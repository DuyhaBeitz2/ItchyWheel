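; BP_FinishLine is a finish line decal with a box trigger that toggles the game's timer when the player crosses it.
; On overlap by player 0's pawn, it finds the BP_Timer actor and calls ToggleGoing, with a DoOnce that resets after a short delay to block rapid re-triggering.
; The construction script picks one of two decal materials based on the Flip90Degrees flag.
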(event OnComponentBeginOverlap(Box)
  (params (OverlappedComponent :type Primitive%20Component%20Object%20Reference) (OtherActor :type Actor%20Object%20Reference) (OtherComp :type Primitive%20Component%20Object%20Reference) (OtherBodyIndex :type Integer) (bFromSweep :type Boolean) (SweepResult :type Hit%20Result%20Structure%20%28by%20ref%29))
  (if (== OtherActor (Game|Player|GetPlayerPawn 0))
    (Utilities|FlowControl|DoOnce false :!label _label
      (:Completed
        (bind _returnvalue (Actor|GetActorOfClass "/Game/BP_Classes/TimeControl/BP_Timer.BP_Timer_C"))
        (Default|ToggleGoing _returnvalue)
        (Utilities|FlowControl|Delay 3.0)
        (goto _label Reset)))))

(event EventBeginPlay)

(event EventTick
  (params (DeltaSeconds :type Float%20%28single-precision%29)))

(fn ConstructionScript
  ;[1 1 1] Decal
  (Rendering|Components|Decal|SetDecalMaterial (Variables|Decal|GetDecal) (select (Variables|Default|GetFlip90Degrees) (Variables|Default|GetMaterial2) (Variables|Default|GetMaterial1))))