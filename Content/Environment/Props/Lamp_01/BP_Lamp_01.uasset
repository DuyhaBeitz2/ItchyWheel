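; BP_Lamp_01 is a lamp prop with a spot light that AI vehicles can knock over.
; UpdateLights runs at construction and BeginPlay, setting light intensity and material emission from BP_Lights_controller's LightsOn flag.
; The first hit by a BP_VehicleAI zeroes emission and the light's source radius (not intensity), enables mesh physics, then destroys the actor after a delay.
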(event OnComponentHit(SM_Lamp_01)
  (params (HitComponent :type Primitive%20Component%20Object%20Reference) (OtherActor :type Actor%20Object%20Reference) (OtherComp :type Primitive%20Component%20Object%20Reference) (NormalImpulse :type Vector :default "0, 0, 0") (Hit :type Hit%20Result%20Structure%20%28by%20ref%29))
  (Utilities|Casting|CastToBP_VehicleAI OtherActor)
  (Utilities|FlowControl|DoOnce false
    (:Completed
      ;[1 1 1] Disable lights
      (Class|PointLightComponent|SetSourceRadius (Variables|Default|GetSpotLight) 0.0)
      (Rendering|Material|SetScalarParameterValueonMaterials (Variables|Default|GetSM_Lamp_01) "LampEmission" 0.0)
      (Physics|SetSimulatePhysics (Variables|Default|GetSM_Lamp_01) true)
      (Utilities|FlowControl|Delay 3.0)
      (Actor|DestroyActor))))

(event EventBeginPlay
  (CallFunction|UpdateLights))

(event Collision|EventActorBeginOverlap
  (params (OtherActor :type Actor%20Object%20Reference)))

(event EventTick
  (params (DeltaSeconds :type Float%20%28single-precision%29)))

(fn ConstructionScript
  (CallFunction|UpdateLights))

(fn UpdateLights
  (bind _returnvalue (Actor|GetActorOfClass "/Game/BP_Classes/Environment/DataControllers/BP_Lights_controller.BP_Lights_controller_C"))
  (Utilities|IsValid _returnvalue
    (:Is%20Valid
      (bind _output_get (Variables|Default|SetLightsOn (Variables|/Game/BP_Classes/Environment/DataControllers/BP_Lights_controller.BP_Lights_controller_C|GetLightsOn _returnvalue)))
      (Rendering|Components|Light|SetIntensity (Variables|Default|GetSpotLight) (* (Math|Conversions|ToFloat(Boolean) _output_get) 1e+05))
      (Rendering|Material|SetScalarParameterValueonMaterials (Variables|Default|GetSM_Lamp_01) "LampEmission" (Math|Conversions|ToFloat(Boolean) _output_get)))))