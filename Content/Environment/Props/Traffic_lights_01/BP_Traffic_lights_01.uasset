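; Traffic light prop that cycles red, yellow and green and controls when BP_VehicleAI cars stop.
; Tick runs timed state changes through DoOnce gates and a FlipFlop, swapping lamp intensities via material parameters.
; The construction script applies the starting state, reversing the FlipFlop order when starting green.
; Each tick, cars in ArriveBox get StopOverride on red or yellow, unless they also overlap LeaveBox.
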(event EventTick
  (params (DeltaSeconds :type Float%20%28single-precision%29))
  (Utilities|FlowControl|Sequence
    (:then_0
      (switch Utilities|FlowControl|Switch|SwitchonE_TrafficLightState (Variables|Default|GetState)
        (:NewEnumerator0
          (Utilities|FlowControl|DoOnce false :!label _label
            (:Completed
              (Utilities|FlowControl|Delay (Variables|Default|GetRedDuration))
              (CallFunction|FromRedtoYellow)
              (goto _label_2 Reset))))
        (:NewEnumerator1
          (Utilities|FlowControl|DoOnce false :!label _label_2
            (:Completed
              (Utilities|FlowControl|Delay (Variables|Default|GetYellowDuration))
              (if (Variables|Default|GetFlipFlopReverse)
                (Utilities|FlowControl|FlipFlop
                  (:A
                    (CallFunction|ToRed)
                    (goto _label Reset))
                  (:B
                    (CallFunction|ToGreen)
                    (goto _label_3 Reset)))
                (else
                  (Utilities|FlowControl|FlipFlop
                    (:A
                      (CallFunction|ToGreen)
                      (goto _label_3 Reset))
                    (:B
                      (CallFunction|ToRed)
                      (goto _label Reset))))))))
        (:NewEnumerator2
          (Utilities|FlowControl|DoOnce false :!label _label_3
            (:Completed
              (Utilities|FlowControl|Delay (Variables|Default|GetGreenDuration))
              (CallFunction|FromGreentoYellow)
              (goto _label_2 Reset))))))
    (:then_1
      (for _array_element (Collision|GetOverlappingActors (Variables|Default|GetArriveBox) "/Game/BP_Classes/Cars/BP_VehicleAI.BP_VehicleAI_C" :!class /Script/Engine.PrimitiveComponent)
        (bind _asbp_vehicle_ai (Utilities|Casting|CastToBP_VehicleAI _array_element))
        (for _array_element_2 (Collision|GetOverlappingActors (Variables|Default|GetLeaveBox) "/Game/BP_Classes/Cars/BP_VehicleAI.BP_VehicleAI_C" :!class /Script/Engine.PrimitiveComponent)
          (if (== _asbp_vehicle_ai _array_element_2)
            (Variables|Default|SetMustlLeave true)
            (Variables|/Game/BP_Classes/Cars/BP_VehicleAI.BP_VehicleAI_C|SetStopOverride _asbp_vehicle_ai false)))
        (if (Variables|Default|GetMustlLeave)
          (Variables|Default|SetMustlLeave false)
          (else
            (switch Utilities|FlowControl|Switch|SwitchonE_TrafficLightState (Variables|Default|GetState)
              (:NewEnumerator0
                (Variables|/Game/BP_Classes/Cars/BP_VehicleAI.BP_VehicleAI_C|SetStopOverride _asbp_vehicle_ai true :!label _label_4)
                (Variables|Default|SetMustlLeave false))
              (:NewEnumerator1
                (goto _label_4))
              (:NewEnumerator2
                (Variables|/Game/BP_Classes/Cars/BP_VehicleAI.BP_VehicleAI_C|SetStopOverride _asbp_vehicle_ai false)
                (Variables|Default|SetMustlLeave false)))))))))

(fn ConstructionScript
  (switch Utilities|FlowControl|Switch|SwitchonE_TrafficLightState (Variables|Default|GetState)
    (:NewEnumerator0
      (CallFunction|ToRed))
    (:NewEnumerator1
      (CallFunction|FromGreentoYellow))
    (:NewEnumerator2
      (CallFunction|ToGreen)
      (Variables|Default|SetFlipFlopReverse true))))

(fn FromGreentoYellow
  ;[1 1 1] Lights
  (Rendering|Material|SetScalarParameterValueonMaterials (Variables|Default|GetStaticMesh) "GreenIntensity" 0.0)
  (Rendering|Material|SetScalarParameterValueonMaterials (Variables|Default|GetStaticMesh) "YellowIntensity" 1e+01)
  (Variables|Default|SetState "NewEnumerator1"))

(fn FromRedtoYellow
  ;[1 1 1] Lights
  (Rendering|Material|SetScalarParameterValueonMaterials (Variables|Default|GetStaticMesh) "RedIntensity" 0.0)
  (Rendering|Material|SetScalarParameterValueonMaterials (Variables|Default|GetStaticMesh) "YellowIntensity" 1e+01)
  (Variables|Default|SetState "NewEnumerator1"))

(fn ToRed
  ;[1 1 1] Lights
  (Rendering|Material|SetScalarParameterValueonMaterials (Variables|Default|GetStaticMesh) "RedIntensity" 1e+01)
  (Rendering|Material|SetScalarParameterValueonMaterials (Variables|Default|GetStaticMesh) "YellowIntensity" 0.0)
  (Variables|Default|SetState "NewEnumerator0"))

(fn ToGreen
  ;[1 1 1] Lights
  (Rendering|Material|SetScalarParameterValueonMaterials (Variables|Default|GetStaticMesh) "GreenIntensity" 1e+01)
  (Rendering|Material|SetScalarParameterValueonMaterials (Variables|Default|GetStaticMesh) "YellowIntensity" 0.0)
  (Variables|Default|SetState "NewEnumerator2"))