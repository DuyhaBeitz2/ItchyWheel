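; Procedural road junction actor that builds a crossroad and up to four straight road arms in its Construction Script, with no runtime logic.
; The connected-road count selects the default, U, T or X junction mesh.
; Each arm places instanced straight meshes at fixed spacing along the actor's forward or right axes, converted to local space.
; Per-road rotations, orientation swaps and an extra yaw for sideways arms correct segment facing.
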(event EventBeginPlay)

(event Collision|EventActorBeginOverlap
  (params (OtherActor :type Actor%20Object%20Reference)))

(event EventTick
  (params (DeltaSeconds :type Float%20%28single-precision%29)))

(fn ConstructionScript
  (bind _returnvalue (Transformation|GetActorRotation))
  (bind _default_crossroad_mesh (Variables|Default|GetDefault_Crossroad_Mesh))
  (bind _returnvalue_2 (* _returnvalue -1.0))
  (bind (_roll _pitch _yaw) (Math|Rotator|BreakRotator _returnvalue_2))
  ;[1 1 1] Crossroad mesh
  (bind _returnvalue_3 (AddComponent|AddStaticMeshComponent false))
  (Transformation|AddRelativeRotation _returnvalue_3 (Variables|Default|GetCrossroad_rotation) false false)
  (Components|StaticMesh|SetStaticMesh _returnvalue_3 (Utilities|Select :Index (Variables|Default|GetNumberOfRoadsConnected) :Option%200 _default_crossroad_mesh :Option%201 _default_crossroad_mesh :Option%202 (Variables|Default|GetU_Shape_Mesh) :Option%203 (Variables|Default|GetT_Shape_Mesh) :Option%204 (Variables|Default|GetX_Shape_Mesh)))
  (Components|StaticMesh|SetStaticMesh (Variables|Default|GetInstanced_straight) (Variables|Default|GetStraightRoadMesh))
  (for _index (range 1 (Variables|Default|GetNumberOfRoadsConnected))
    (for _index_2 (range 1 (Utilities|Select :Index _index :Option%200 0 :Option%201 (Variables|Default|GetFirst_road_length) :Option%202 (Variables|Default|GetSecond_road_length) :Option%203 (Variables|Default|GetThird_road_length) :Option%204 (Variables|Default|GetFourth_road_length)))
      (Utilities|FlowControl|Sequence
        (:then_0
          (CallFunction|ResetNewTransform)
          (Variables|Default|SetNewLocationRelative (* (Math|Vector|RotateVector (Utilities|Select :Index _index :Option%200 "0, 0, 0" :Option%201 (* (Transformation|GetActorForwardVector) (Variables|Default|GetFirstRoatDirection)) :Option%202 (* (Transformation|GetActorRightVector) (Variables|Default|GetSecondRoadDirection)) :Option%203 (* (Transformation|GetActorForwardVector) -1 (Variables|Default|GetFirstRoatDirection)) :Option%204 (* (Transformation|GetActorRightVector) (Variables|Default|GetSecondRoadDirection) -1)) (Math|Rotator|MakeRotator _roll _pitch _yaw)) 800 _index_2))
          (CallFunction|AddRotationtoNewRelativeRotation (Utilities|Select :Index _index :Option%200 "0, 0, 0" :Option%201 (Variables|Rotation|GetFirst_road_rotation) :Option%202 (Variables|Rotation|GetSecond_road_rotation) :Option%203 (Variables|Rotation|GetThird_road_rotation) :Option%204 (Variables|Rotation|GetFourth_road_rotation)))
          (if (or (Utilities|Operators|EqualEqual (Math|Vector|RotateVector (Transformation|GetActorRightVector) (* (Transformation|GetActorRotation) -1.0)) (Math|Vector|RotateVector (Utilities|Select :Index _index :Option%200 "0, 0, 0" :Option%201 (* (Transformation|GetActorForwardVector) (Variables|Default|GetFirstRoatDirection)) :Option%202 (* (Transformation|GetActorRightVector) (Variables|Default|GetSecondRoadDirection)) :Option%203 (* (Transformation|GetActorForwardVector) -1 (Variables|Default|GetFirstRoatDirection)) :Option%204 (* (Transformation|GetActorRightVector) (Variables|Default|GetSecondRoadDirection) -1)) (Math|Rotator|MakeRotator _roll _pitch _yaw)) 0.05) (Utilities|Operators|EqualEqual (Math|Vector|RotateVector (Utilities|Select :Index _index :Option%200 "0, 0, 0" :Option%201 (* (Transformation|GetActorForwardVector) (Variables|Default|GetFirstRoatDirection)) :Option%202 (* (Transformation|GetActorRightVector) (Variables|Default|GetSecondRoadDirection)) :Option%203 (* (Transformation|GetActorForwardVector) -1 (Variables|Default|GetFirstRoatDirection)) :Option%204 (* (Transformation|GetActorRightVector) (Variables|Default|GetSecondRoadDirection) -1)) (Math|Rotator|MakeRotator _roll _pitch _yaw)) (* (Math|Vector|RotateVector (Transformation|GetActorRightVector) (* (Transformation|GetActorRotation) -1.0)) -1) 0.05))
            (CallFunction|AddRotationtoNewRelativeRotation (Math|Rotator|MakeRotator 0.0 0.0 (Math|Conversions|ToFloat(Integer) (* (Variables|Default|GetOrientations) 90)))))
          (if (Variables|Swap|GetSwapOrientations)
            (CallFunction|AddRotationtoNewRelativeRotation (Math|Rotator|MakeRotator 0.0 0.0 9e+01)))
          (if (and (or (Utilities|Operators|EqualEqual (Math|Vector|RotateVector (Transformation|GetActorRightVector) (* (Transformation|GetActorRotation) -1.0)) (Math|Vector|RotateVector (Utilities|Select :Index _index :Option%200 "0, 0, 0" :Option%201 (* (Transformation|GetActorForwardVector) (Variables|Default|GetFirstRoatDirection)) :Option%202 (* (Transformation|GetActorRightVector) (Variables|Default|GetSecondRoadDirection)) :Option%203 (* (Transformation|GetActorForwardVector) -1 (Variables|Default|GetFirstRoatDirection)) :Option%204 (* (Transformation|GetActorRightVector) (Variables|Default|GetSecondRoadDirection) -1)) (Math|Rotator|MakeRotator _roll _pitch _yaw)) 0.05) (Utilities|Operators|EqualEqual (Math|Vector|RotateVector (Utilities|Select :Index _index :Option%200 "0, 0, 0" :Option%201 (* (Transformation|GetActorForwardVector) (Variables|Default|GetFirstRoatDirection)) :Option%202 (* (Transformation|GetActorRightVector) (Variables|Default|GetSecondRoadDirection)) :Option%203 (* (Transformation|GetActorForwardVector) -1 (Variables|Default|GetFirstRoatDirection)) :Option%204 (* (Transformation|GetActorRightVector) (Variables|Default|GetSecondRoadDirection) -1)) (Math|Rotator|MakeRotator _roll _pitch _yaw)) (* (Math|Vector|RotateVector (Transformation|GetActorRightVector) (* (Transformation|GetActorRotation) -1.0)) -1) 0.05)) (Variables|Swap|GetSwapRightOrientations))
            (CallFunction|AddRotationtoNewRelativeRotation (Math|Rotator|MakeRotator 0.0 0.0 9e+01))))
        (:then_1
          (CallFunction|AddStraightRoadInstance))))))

(fn AddRotationtoNewRelativeRotation
  (params (Rotator :type Rotator))
  (Variables|Default|SetNewRotationRelative (Math|Rotator|CombineRotators Rotator (Variables|Default|GetNewRotationRelative))))

(fn AddStraightRoadInstance
  (Components|InstancedStaticMesh|AddInstance (Variables|Default|GetInstanced_straight) (Math|Transform|MakeTransform (Variables|Default|GetNewLocationRelative) (Variables|Default|GetNewRotationRelative) "1.000000,1.000000,1.000000") false))

(fn ResetNewTransform
  (Variables|Default|SetNewLocationRelative "0, 0, 0")
  (Variables|Default|SetNewRotationRelative "0, 0, 0"))