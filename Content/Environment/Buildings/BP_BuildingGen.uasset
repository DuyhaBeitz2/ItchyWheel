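; Procedural building actor that stacks modular floor meshes in the construction script, topped with a roof and an occasional water tower.
; Random generation picks floor count, meshes and one shared brick material, offsetting each piece by the previous mesh's bounds height.
; It records the layout so that enabling Save rebuilds the same building instead of rerolling.
; UpdateLights copies BP_Lights_controller's LightsOn into window emission at construction and BeginPlay.
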(event EventBeginPlay
  (CallFunction|UpdateLights))

(event Collision|EventActorBeginOverlap
  (params (OtherActor :type Actor%20Object%20Reference)))

(event EventTick
  (params (DeltaSeconds :type Float%20%28single-precision%29)))

(fn ConstructionScript
  (Utilities|FlowControl|Sequence
    (:then_0
      (if (Variables|Default|GetSave)
        (Variables|Default|SetPreviousFloorHeight 0.0)
        (for (_ _array_index) (Variables|Default|GetSavedFloorVector)
          (CallFunction|NewFloor (Utilities|Array|MakeArray (Utilities|Array|Get(acopy) (Variables|Default|GetSavedFloorVector) _array_index)) (Math|Transform|MakeTransform (+ (Variables|Default|GetPreviousLocation) (Math|Vector|MakeVector 0.0 0.0 (Variables|Default|GetPreviousFloorHeight)))) (Variables|Default|GetSavedColorIndex))
          (CallFunction|SaveFloor))
        ;[1 1 1] Roof
        (bind _returnvalue (AddComponent|AddStaticMeshComponent false (Math|Transform|MakeTransform (+ (Variables|Default|GetPreviousLocation) (Math|Vector|MakeVector 0.0 0.0 (Variables|Default|GetPreviousFloorHeight))))))
        (bind _output_get (Variables|Default|SetNewMesh _returnvalue))
        (Components|StaticMesh|SetStaticMesh _output_get (Variables|Default|GetRoofMesh))
        (if (Variables|Default|GetSavedWaterTower)
          (bind _returnvalue_2 (AddComponent|AddStaticMeshComponent false (Math|Transform|MakeTransform (+ (Variables|Default|GetPreviousLocation) (Math|Vector|MakeVector 3e+02 0.0 (Variables|Default|GetPreviousFloorHeight))))))
          (bind _output_get_2 (Variables|Default|SetNewMesh _returnvalue_2))
          (Components|StaticMesh|SetStaticMesh _output_get_2 "/Game/Environment/Props/WaterTower/SM_WaterTower_01.SM_WaterTower_01"))
        (else
          (Variables|Default|SetColorIndex (Math|Random|RandomIntegerinRange 0 4))
          (bind _output_get_3 (Variables|Default|SetFloors (Math|Random|RandomIntegerinRange 2 (Variables|Default|GetMaxHeight))))
          (for _index (range 0 _output_get_3)
            ;[1 1 1] Generate FirstFloor
            (if (== _index 0)
              (CallFunction|NewFloor (Variables|Default|GetFirstFloorMeshes) (Math|Transform|MakeTransform "0, 0, 0") (Variables|Default|GetColorIndex))
              (CallFunction|SaveFloor)
              (else
                ;[1 1 1] MiddleFloors
                (CallFunction|NewFloor (Variables|Default|GetMiddleFloorMeshes) (Math|Transform|MakeTransform (+ (Variables|Default|GetPreviousLocation) (Math|Vector|MakeVector 0.0 0.0 (Variables|Default|GetPreviousFloorHeight)))) (Variables|Default|GetColorIndex))
                (CallFunction|SaveFloor))))
          ;[1 1 1] Roof
          (bind _returnvalue_3 (AddComponent|AddStaticMeshComponent false (Math|Transform|MakeTransform (+ (Variables|Default|GetPreviousLocation) (Math|Vector|MakeVector 0.0 0.0 (Variables|Default|GetPreviousFloorHeight))))))
          (bind _output_get_4 (Variables|Default|SetNewMesh _returnvalue_3))
          (Components|StaticMesh|SetStaticMesh _output_get_4 (Variables|Default|GetRoofMesh))
          (Variables|Default|SetSavedFloorVector (Variables|Default|GetFloorVector))
          (Utilities|Array|Clear (Variables|Default|GetFloorVector))
          (Variables|Default|SetSavedColorIndex (Variables|Default|GetColorIndex))
          ;[1 1 1] Add water tower
          (Variables|Default|SetSavedWaterTower false)
          (if (and (Math|Random|RandomBool) (Math|Random|RandomBool))
            (bind _returnvalue_4 (AddComponent|AddStaticMeshComponent false (Math|Transform|MakeTransform (+ (Variables|Default|GetPreviousLocation) (Math|Vector|MakeVector 3e+02 0.0 (Variables|Default|GetPreviousFloorHeight))))))
            (bind _output_get_5 (Variables|Default|SetNewMesh _returnvalue_4))
            (Components|StaticMesh|SetStaticMesh _output_get_5 "/Game/Environment/Props/WaterTower/SM_WaterTower_01.SM_WaterTower_01")
            (Variables|Default|SetSavedWaterTower true)))))
    (:then_1
      (CallFunction|UpdateLights))))

(fn ChooseColor
  (params (ColorIndex :type Integer))
  (return (Utilities|Select :Index ColorIndex :Option%200 "/Game/Environment/Buildings/Elements/Walls/Bricks_01/MI_Bricks_01.MI_Bricks_01" :Option%201 "/Game/Environment/Buildings/Elements/Walls/Bricks_02/MI_Bricks_02.MI_Bricks_02" :Option%202 "/Game/Environment/Buildings/Elements/Walls/Bricks_03/MI_Bricks_03.MI_Bricks_03" :Option%203 "/Game/Environment/Buildings/Elements/Walls/Bricks_04/MI_Bricks_04.MI_Bricks_04" :Option%204 "/Game/Environment/Buildings/Elements/Walls/Bricks_05/MI_Bricks_05.MI_Bricks_05")))

(fn NewFloor
  (params (PossibleMeshes :type Array%20of%20Static%20Mesh%20Object%20References) (Transform :type Transform) (ColorIndex :type Integer))
  (bind _returnvalue (AddComponent|AddStaticMeshComponent false Transform))
  (bind _output_get (Variables|Default|SetNewMesh _returnvalue))
  (Components|StaticMesh|SetStaticMesh _output_get (.OutItem (Utilities|Array|Random PossibleMeshes)))
  (bind _material (CallFunction|ChooseColor ColorIndex))
  (Rendering|Material|SetMaterialbyName _output_get "BaseColor" _material)
  (Rendering|Material|SetScalarParameterValueonMaterials _output_get "EmissionFactor" (Math|Conversions|ToFloat(Boolean) (Variables|Default|GetLightsOn))))

(fn SaveHeight
  (Variables|Default|SetPreviousFloorHeight (.Z (Math|Vector|BreakVector (.Max (Components|StaticMesh|GetLocalBounds (Variables|Default|GetNewMesh)))))))

(fn SaveLocation
  (Variables|Default|SetPreviousLocation (Variables|/Script/Engine.SceneComponent|GetRelativeLocation (Variables|Default|GetNewMesh))))

(fn SaveMeshforBaking
  (Utilities|Array|Add (Variables|Default|GetFloorVector) (Variables|/Script/Engine.StaticMeshComponent|GetStaticMesh (Variables|Default|GetNewMesh))))

(fn SaveFloor
  ;[1 1 1] Save
  (CallFunction|SaveHeight)
  (CallFunction|SaveLocation)
  (CallFunction|SaveMeshforBaking))

(fn UpdateLights
  (bind _returnvalue (Actor|GetActorOfClass "/Game/BP_Classes/Environment/BP_Lights_controller.BP_Lights_controller_C"))
  (Utilities|IsValid _returnvalue
    (:Is%20Valid
      (Variables|Default|SetLightsOn (Variables|/Game/BP_Classes/Environment/BP_Lights_controller.BP_Lights_controller_C|GetLightsOn _returnvalue))
      (for _array_element (Actor|GetComponentsByClass "/Script/Engine.StaticMeshComponent")
        (Rendering|Material|SetScalarParameterValueonMaterials _array_element "WindowEmission" (Math|Conversions|ToFloat(Boolean) (Variables|Default|GetLightsOn)))))))