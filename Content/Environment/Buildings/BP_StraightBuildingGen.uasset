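; Procedural building generator that assembles a straight stack of floor meshes in its Construction Script.
; With Save off, it stacks a first floor, random middle floors up to MaxHeight and a roof, using one random brick material and an occasional water tower.
; Each piece sits atop the previous mesh's bounds height.
; It records meshes, color and water tower choice, so turning Save on rebuilds that layout instead of rerolling.
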(event EventBeginPlay)

(event Collision|EventActorBeginOverlap
  (params (OtherActor :type Actor%20Object%20Reference)))

(event EventTick
  (params (DeltaSeconds :type Float%20%28single-precision%29)))

(fn ConstructionScript
  (if (Variables|Default|GetSave)
    (Variables|Default|SetPreviousFloorHeight 0.0)
    (for (_ _array_index) (Variables|Default|GetSavedFloorVector)
      (bind _returnvalue (AddComponent|AddStaticMeshComponent false (Math|Transform|MakeTransform (+ (Variables|Default|GetPreviousLocation) (Math|Vector|MakeVector 0.0 0.0 (Variables|Default|GetPreviousFloorHeight))))))
      (bind _output_get (Variables|Default|SetNewMesh _returnvalue))
      (Components|StaticMesh|SetStaticMesh _output_get (Utilities|Array|Get(acopy) (Variables|Default|GetSavedFloorVector) _array_index))
      ;[1 1 1] Color
      (bind _material (CallFunction|ChooseColor (Variables|Default|GetSavedColorIndex)))
      (Rendering|Material|SetMaterialbyName (Variables|Default|GetNewMesh) "BaseColor" _material)
      ;[1 1 1] SaveHeight
      (Variables|Default|SetPreviousFloorHeight (.Z (Math|Vector|BreakVector (.Max (Components|StaticMesh|GetLocalBounds (Variables|Default|GetNewMesh))))))
      ;[1 1 1] Save location
      (Variables|Default|SetPreviousLocation (Variables|/Script/Engine.SceneComponent|GetRelativeLocation (Variables|Default|GetNewMesh))))
    ;[1 1 1] Roof
    (bind _returnvalue_2 (AddComponent|AddStaticMeshComponent false (Math|Transform|MakeTransform (+ (Variables|Default|GetPreviousLocation) (Math|Vector|MakeVector 0.0 0.0 (Variables|Default|GetPreviousFloorHeight))))))
    (bind _output_get_2 (Variables|Default|SetNewMesh _returnvalue_2))
    (Components|StaticMesh|SetStaticMesh _output_get_2 "/Game/Environment/Buildings/GenericFloors/Straight/Roofs/Roof_01/SM_Roof_01.SM_Roof_01")
    (if (Variables|Default|GetSavedWaterTower)
      (bind _returnvalue_3 (AddComponent|AddStaticMeshComponent false (Math|Transform|MakeTransform (+ (Variables|Default|GetPreviousLocation) (Math|Vector|MakeVector 3e+02 0.0 (Variables|Default|GetPreviousFloorHeight))))))
      (bind _output_get_3 (Variables|Default|SetNewMesh _returnvalue_3))
      (Components|StaticMesh|SetStaticMesh _output_get_3 "/Game/Environment/Props/WaterTower/SM_WaterTower_01.SM_WaterTower_01"))
    (else
      (Variables|Default|SetColorIndex (Math|Random|RandomIntegerinRange 0 4))
      (bind _output_get_4 (Variables|Default|SetFloors (Math|Random|RandomIntegerinRange 2 (Variables|Default|GetMaxHeight))))
      (for _index (range 0 _output_get_4)
        ;[1 1 1] FirstFloor
        (if (== _index 0)
          (bind _returnvalue_4 (AddComponent|AddStaticMeshComponent false))
          (bind _output_get_5 (Variables|Default|SetNewMesh _returnvalue_4))
          (Components|StaticMesh|SetStaticMesh _output_get_5 "/Game/Environment/Buildings/GenericFloors/Straight/First/FirstFloor_01/FirstFloor_01.FirstFloor_01")
          (bind _material_2 (CallFunction|ChooseColor (Variables|Default|GetColorIndex)))
          (Rendering|Material|SetMaterialbyName _output_get_5 "BaseColor" _material_2)
          ;[1 1 1] SaveHeight
          (Variables|Default|SetPreviousFloorHeight (.Z (Math|Vector|BreakVector (.Max (Components|StaticMesh|GetLocalBounds (Variables|Default|GetNewMesh))))))
          ;[1 1 1] Save location
          (Variables|Default|SetPreviousLocation (Variables|/Script/Engine.SceneComponent|GetRelativeLocation (Variables|Default|GetNewMesh)))
          ;[1 1 1] Save mesh for baking
          (Utilities|Array|Add (Variables|Default|GetFloorVector) (Variables|/Script/Engine.StaticMeshComponent|GetStaticMesh (Variables|Default|GetNewMesh)))
          (else
            ;[1 1 1] MiddleFloors
            (bind _returnvalue_5 (AddComponent|AddStaticMeshComponent false (Math|Transform|MakeTransform (+ (Variables|Default|GetPreviousLocation) (Math|Vector|MakeVector 0.0 0.0 (Variables|Default|GetPreviousFloorHeight))))))
            (bind _output_get_6 (Variables|Default|SetNewMesh _returnvalue_5))
            (Components|StaticMesh|SetStaticMesh _output_get_6 (select (Math|Random|RandomBool) "/Game/Environment/Buildings/GenericFloors/Straight/Middle/Middle_02/SM_MiddleFloor_02.SM_MiddleFloor_02" "/Game/Environment/Buildings/GenericFloors/Straight/Middle/Middle_01/SM_MiddleFloor_01.SM_MiddleFloor_01"))
            (bind _material_3 (CallFunction|ChooseColor (Variables|Default|GetColorIndex)))
            (Rendering|Material|SetMaterialbyName _output_get_6 "BaseColor" _material_3)
            ;[1 1 1] SaveHeight
            (Variables|Default|SetPreviousFloorHeight (.Z (Math|Vector|BreakVector (.Max (Components|StaticMesh|GetLocalBounds (Variables|Default|GetNewMesh))))))
            ;[1 1 1] Save location
            (Variables|Default|SetPreviousLocation (Variables|/Script/Engine.SceneComponent|GetRelativeLocation (Variables|Default|GetNewMesh)))
            ;[1 1 1] Save mesh for baking
            (Utilities|Array|Add (Variables|Default|GetFloorVector) (Variables|/Script/Engine.StaticMeshComponent|GetStaticMesh (Variables|Default|GetNewMesh))))))
      ;[1 1 1] Roof
      (bind _returnvalue_6 (AddComponent|AddStaticMeshComponent false (Math|Transform|MakeTransform (+ (Variables|Default|GetPreviousLocation) (Math|Vector|MakeVector 0.0 0.0 (Variables|Default|GetPreviousFloorHeight))))))
      (bind _output_get_7 (Variables|Default|SetNewMesh _returnvalue_6))
      (Components|StaticMesh|SetStaticMesh _output_get_7 "/Game/Environment/Buildings/GenericFloors/Straight/Roofs/Roof_01/SM_Roof_01.SM_Roof_01")
      (Variables|Default|SetSavedFloorVector (Variables|Default|GetFloorVector))
      (Utilities|Array|Clear (Variables|Default|GetFloorVector))
      (Variables|Default|SetSavedColorIndex (Variables|Default|GetColorIndex))
      ;[1 1 1] Add water tower
      (Variables|Default|SetSavedWaterTower false)
      (if (and (Math|Random|RandomBool) (Math|Random|RandomBool))
        (bind _returnvalue_7 (AddComponent|AddStaticMeshComponent false (Math|Transform|MakeTransform (+ (Variables|Default|GetPreviousLocation) (Math|Vector|MakeVector 3e+02 0.0 (Variables|Default|GetPreviousFloorHeight))))))
        (bind _output_get_8 (Variables|Default|SetNewMesh _returnvalue_7))
        (Components|StaticMesh|SetStaticMesh _output_get_8 "/Game/Environment/Props/WaterTower/SM_WaterTower_01.SM_WaterTower_01")
        (Variables|Default|SetSavedWaterTower true)))))

(fn ChooseColor
  (params (ColorIndex :type Integer))
  (return (Utilities|Select :Index ColorIndex :Option%200 "/Game/Environment/Buildings/Elements/Walls/Bricks_01/MI_Bricks_01.MI_Bricks_01" :Option%201 "/Game/Environment/Buildings/Elements/Walls/Bricks_02/MI_Bricks_02.MI_Bricks_02" :Option%202 "/Game/Environment/Buildings/Elements/Walls/Bricks_03/MI_Bricks_03.MI_Bricks_03" :Option%203 "/Game/Environment/Buildings/Elements/Walls/Bricks_04/MI_Bricks_04.MI_Bricks_04" :Option%204 "/Game/Environment/Buildings/Elements/Walls/Bricks_05/MI_Bricks_05.MI_Bricks_05")))