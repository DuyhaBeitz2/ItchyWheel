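; Fountain actor that shows a water effect and launches wheeled vehicles along its up axis while active.
; Each tick, a sphere trace along that axis finds a vehicle and applies a velocity-change impulse, inversely proportional to hit distance and capped at MaxForce.
; The construction script sets the effect's spawn rate.
; After Duration from BeginPlay, the spawn rate drops to zero and the force switches off.
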(event EventBeginPlay
  (Utilities|FlowControl|Delay (Variables|Default|GetDuration))
  (Variables|Default|SetSpawnRate 0.0)
  (Variables|Default|SetAppliesForce false)
  (Niagara|SetNiagaraVariable(Float) (Variables|Default|GetN_Water) "SpawnRate" (Variables|Default|GetSpawnRate)))

(event Collision|EventActorBeginOverlap
  (params (OtherActor :type Actor%20Object%20Reference)))

(event EventTick
  (params (DeltaSeconds :type Float%20%28single-precision%29))
  (bind _returnvalue (Transformation|GetActorLocation))
  (if (Variables|Default|GetAppliesForce)
    (bind _outhit (Collision|SphereTraceForObjects _returnvalue (+ _returnvalue (* (Transformation|GetActorUpVector) (Variables|Default|GetHeight))) 75.0 (Utilities|Array|MakeArray "ObjectTypeQuery5" "ObjectTypeQuery3" "ObjectTypeQuery4") false 0 "None"))
    (bind _aswheeled_vehicle_pawn (Utilities|Casting|CastToWheeledVehiclePawn (.HitActor (Collision|BreakHitResult _outhit))))
    ;[1 1 1] Make sure force is never too high
    (if (> (Math|Vector|VectorLength (/ (* (Transformation|GetActorUpVector) (Variables|Default|GetForce)) (Math|Vector|VectorLength (- (.ImpactPoint (Collision|BreakHitResult _outhit)) (Transformation|GetActorLocation))))) (Variables|Default|GetMaxForce))
      (Physics|AddImpulse (Variables|/Script/ChaosVehicles.WheeledVehiclePawn|GetMesh _aswheeled_vehicle_pawn) (* (Math|Vector|Normalize (/ (* (Transformation|GetActorUpVector) (Variables|Default|GetForce)) (Math|Vector|VectorLength (- (.ImpactPoint (Collision|BreakHitResult _outhit)) (Transformation|GetActorLocation))))) (Variables|Default|GetMaxForce)) "Root" true)
      (else
        (Physics|AddImpulse (Variables|/Script/ChaosVehicles.WheeledVehiclePawn|GetMesh _aswheeled_vehicle_pawn) (/ (* (Transformation|GetActorUpVector) (Variables|Default|GetForce)) (Math|Vector|VectorLength (- (.ImpactPoint (Collision|BreakHitResult _outhit)) (Transformation|GetActorLocation)))) "Root" true)))))

(fn ConstructionScript
  (Niagara|SetNiagaraVariable(Float) (Variables|Default|GetN_Water) "SpawnRate" (Variables|Default|GetSpawnRate)))