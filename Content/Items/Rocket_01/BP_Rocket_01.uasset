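; BP_Rocket_01 is a pickup that gives the player's vehicle a timed rocket boost when overlapped.
; It flags the vehicle as boosted, sets its forward boost vector, and attaches a spawned rocket mesh with glowing emission and Niagara fire.
; After the duration, it clears the flag and flings the rocket sideways, based on the road side, and upward with gravity disabled, then destroys everything after a delay.
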(event OnComponentBeginOverlap(Sphere)
  (params (OverlappedComponent :type Primitive%20Component%20Object%20Reference) (OtherActor :type Actor%20Object%20Reference) (OtherComp :type Primitive%20Component%20Object%20Reference) (OtherBodyIndex :type Integer) (bFromSweep :type Boolean) (SweepResult :type Hit%20Result%20Structure%20%28by%20ref%29))
  ;[1 1 1] On overlap
  (if (== OtherActor (Game|Player|GetPlayerPawn 0))
    (bind _asbp_vehicle_ai (Utilities|Casting|CastToBP_VehicleAI OtherActor))
    (bind _output_get (Variables|Default|SetPlayerVehicle _asbp_vehicle_ai))
    ;[1 1 1] Boost
    (Variables|/Game/BP_Classes/Cars/BP_VehicleAI.BP_VehicleAI_C|SetIsBoostApplied _output_get true)
    (Variables|/Game/BP_Classes/Cars/BP_VehicleAI.BP_VehicleAI_C|SetBoost _asbp_vehicle_ai (* (Transformation|GetActorForwardVector _asbp_vehicle_ai) (Variables|Default|GetBoost)))
    ;[1 1 1] Spawn rocket mesh actor
    (bind _returnvalue (Game|SpawnActorfromClass "/Script/Engine.StaticMeshActor" (Math|Transform|MakeTransform "0, 0, 0") "AlwaysSpawn" "MultiplyWithRoot" (Game|GetPlayerController 0) 0))
    (bind _output_get_2 (Variables|Default|SetNewMeshActor _returnvalue))
    (Transformation|SetMobility _output_get_2 "Movable")
    (Transformation|AttachActorToActor (Variables|Default|GetNewMeshActor) (Variables|Default|GetPlayerVehicle) "RocketSocket" "SnapToTarget" "SnapToTarget" "SnapToTarget" false)
    ;[1 1 1] Setup mesh asset
    (bind _output_get_3 (Variables|Default|SetNewMeshComponent (Variables|/Script/Engine.StaticMeshActor|GetStaticMeshComponent (Variables|Default|GetNewMeshActor))))
    (Components|StaticMesh|SetStaticMesh _output_get_3 (Variables|/Script/Engine.StaticMeshComponent|GetStaticMesh (Variables|Default|GetSKM_Rocket_01)))
    (Collision|SetCollisionResponsetoChannel (Variables|Default|GetNewMeshComponent) "ECC_Camera" "ECR_Ignore")
    (Collision|SetCollisionResponsetoChannel (Variables|Default|GetNewMeshComponent) "ECC_Vehicle" "ECR_Ignore")
    ;[1 1 1] Add glowing emission to rocket
    (Rendering|Material|SetScalarParameterValueonMaterials (Variables|Default|GetNewMeshComponent) "Emission" 3e+02)
    ;[1 1 1] Add fire
    (bind _returnvalue_2 (Niagara|SpawnSystemAttached "/Game/FX/Fire/N_Fire.N_Fire" (Variables|Default|GetNewMeshComponent) "FireSocket" "0, 0, 0" "90.000000,0.000000,0.000000" "KeepRelativeOffset" false))
    (Variables|Default|SetNewNiagra _returnvalue_2)
    ;[1 1 1] Boost ended
    (Utilities|FlowControl|Delay (Variables|Default|GetDuration))
    (Transformation|DetachFromComponent (Variables|Default|GetNewMeshComponent) "KeepWorld" "KeepWorld" "KeepWorld" false)
    (Physics|SetSimulatePhysics (Variables|Default|GetNewMeshComponent) true)
    (Physics|AddImpulse (Variables|Default|GetNewMeshComponent) (* (+ (* (Transformation|GetActorRightVector (Variables|Default|GetPlayerVehicle)) (Variables|/Game/BP_Classes/Cars/BP_VehicleAI.BP_VehicleAI_C|GetSideOfRoad (Variables|Default|GetPlayerVehicle))) (Transformation|GetActorUpVector (Variables|Default|GetPlayerVehicle))) 420) "None" true)
    (Class|PrimitiveComponent|AddAngularImpulseinDegrees (Variables|Default|GetNewMeshComponent) (* (Transformation|GetActorRightVector (Variables|Default|GetPlayerVehicle)) 1.5e+02 (Variables|/Game/BP_Classes/Cars/BP_VehicleAI.BP_VehicleAI_C|GetSideOfRoad (Variables|Default|GetPlayerVehicle))) "None" true)
    (Physics|SetEnableGravity (Variables|Default|GetNewMeshComponent) false)
    (Variables|/Game/BP_Classes/Cars/BP_VehicleAI.BP_VehicleAI_C|SetIsBoostApplied (Variables|Default|GetPlayerVehicle) false)
    ;[1 1 1] Destroy
    (Utilities|FlowControl|Delay 6.0)
    (Components|DestroyComponent (Variables|Default|GetNewNiagra))
    (Actor|DestroyActor (Variables|Default|GetNewMeshActor))
    (Actor|DestroyActor)))

(event EventBeginPlay
  (|CallParentFunction) ; This node is disabled and will not be called.\nDrag off pins to build functionality.
)

(event Collision|EventActorBeginOverlap
  (params (OtherActor :type Actor%20Object%20Reference))
  (|CallParentFunction OtherActor) ; This node is disabled and will not be called.\nDrag off pins to build functionality.
)

(event EventTick
  (params (DeltaSeconds :type Float%20%28single-precision%29))
  (|CallParentFunction DeltaSeconds) ; This node is disabled and will not be called.\nDrag off pins to build functionality.
)

(fn ConstructionScript
  (|CallParentFunction))