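; Player-controllable taxi passenger car Blueprint that adds Enhanced Input setup and camera look to its parent class.
; On BeginPlay it calls the parent, then registers the IMC_Main mapping context with the local player subsystem when a PlayerController possesses it.
; The IA_LookAround action feeds controller yaw and pitch for looking around.
; Tick, overlap and construction script add no logic of their own.
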(event Input|EnhancedActionEvents|EnhancedInputActionIA_LookAround
  (params (ActionValue :type Vector%202D%20Structure) (ElapsedSeconds :type Float%20%28double-precision%29) (TriggeredSeconds :type Float%20%28double-precision%29) (InputAction :type Input%20Action%20Object%20Reference :default "/Game/Input/Test/IA_LookAround.IA_LookAround"))
  (bind (_x _y) (Math|Vector2D|BreakVector2D ActionValue))
  ;[1 1 1] Look Around
  (Pawn|Input|AddControllerYawInput _x)
  (Pawn|Input|AddControllerPitchInput _y))

(event EventBeginPlay
  ;[1 1 1] Add mapping context
  (|CallParentFunction)
  (bind _asplayer_controller (Utilities|Casting|CastToPlayerController (Pawn|GetController)))
  (Input|AddMappingContext (PlayerController|LocalPlayerSubsystems|GetEnhancedInputLocalPlayerSubsystem _asplayer_controller) "/Game/Input/Main/IMC_Main.IMC_Main" 0 "(bIgnoreAllPressedKeysUntilRelease=True,bForceImmediately=False,bNotifyUserSettings=False)"))

(event Collision|EventActorBeginOverlap
  (params (OtherActor :type Actor%20Object%20Reference)))

(event EventTick
  (params (DeltaSeconds :type Float%20%28single-precision%29))
  (|CallParentFunction DeltaSeconds) ; This node is disabled and will not be called.\nDrag off pins to build functionality.
)

(fn ConstructionScript
  (|CallParentFunction))