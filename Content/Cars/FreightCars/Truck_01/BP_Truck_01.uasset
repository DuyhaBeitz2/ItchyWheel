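; Player-controlled freight truck vehicle that maps Enhanced Input to throttle, handbrake, camera look, pause and road-side selection.
; Left and right inputs step SideOfRoad between -1 and 1, extend it to an outer ±3 while triggered, and pull it back on release.
; BeginPlay, Tick and construction defer to the parent class, and this graph only sets SideOfRoad without steering.
; Debug keys open level selection, print save slot names and reload the last played level.
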(event Input|EnhancedActionEvents|EnhancedInputActionIA_LookAround
  (params (ActionValue :type Vector%202D%20Structure) (ElapsedSeconds :type Float%20%28double-precision%29) (TriggeredSeconds :type Float%20%28double-precision%29) (InputAction :type Input%20Action%20Object%20Reference :default "/Game/Input/Test/IA_LookAround.IA_LookAround"))
  (bind (_x _y) (Math|Vector2D|BreakVector2D ActionValue))
  ;[1 1 1] Look Around
  (Pawn|Input|AddControllerYawInput _x)
  (Pawn|Input|AddControllerPitchInput _y))

(event Input|EnhancedActionEvents|EnhancedInputActionIA_Pause
  (params (ActionValue :type Boolean) (ElapsedSeconds :type Float%20%28double-precision%29) (TriggeredSeconds :type Float%20%28double-precision%29) (InputAction :type Input%20Action%20Object%20Reference :default "/Game/Input/Test/IA_Pause.IA_Pause"))
  (CallFunction|PauseUnpause))

(event Input|EnhancedActionEvents|EnhancedInputActionIA_Handbrake
  (params (ActionValue :type Boolean) (ElapsedSeconds :type Float%20%28double-precision%29) (TriggeredSeconds :type Float%20%28double-precision%29) (InputAction :type Input%20Action%20Object%20Reference :default "/Game/Input/Test/IA_Handbrake.IA_Handbrake"))
  ;[1 1 1] Handbrake
  (:Triggered
    (Class|ChaosVehicleMovementComponent|SetHandbrakeInput (Variables|Default|GetVehicleMovementComponent) true))
  (:Canceled
    (Class|ChaosVehicleMovementComponent|SetHandbrakeInput (Variables|Default|GetVehicleMovementComponent) false :!label _label))
  (:Completed
    (goto _label)))

(event Input|EnhancedActionEvents|EnhancedInputActionIA_LeftSideOfRoad
  (params (ActionValue :type Boolean) (ElapsedSeconds :type Float%20%28double-precision%29) (TriggeredSeconds :type Float%20%28double-precision%29) (InputAction :type Input%20Action%20Object%20Reference :default "/Game/Input/Test/IA_LeftSideOfRoad.IA_LeftSideOfRoad"))
  (:Triggered
    (if (== (Variables|Default|GetSideOfRoad) -1)
      (Variables|Default|SetSideOfRoad -3)))
  (:Started
    (Variables|Default|SetSideOfRoad (Math|Integer|Max(Integer) (+ (Variables|Default|GetSideOfRoad) -2) -1)))
  (:Canceled
    (Variables|Default|SetSideOfRoad (Math|Integer|Max(Integer) (Variables|Default|GetSideOfRoad) -1) :!label _label))
  (:Completed
    (goto _label)))

(event Input|EnhancedActionEvents|EnhancedInputActionIA_RightSideOfRoad
  (params (ActionValue :type Boolean) (ElapsedSeconds :type Float%20%28double-precision%29) (TriggeredSeconds :type Float%20%28double-precision%29) (InputAction :type Input%20Action%20Object%20Reference :default "/Game/Input/Test/IA_RightSideOfRoad.IA_RightSideOfRoad"))
  (:Triggered
    (if (== (Variables|Default|GetSideOfRoad) 1)
      (Variables|Default|SetSideOfRoad 3)))
  (:Started
    (Variables|Default|SetSideOfRoad (Math|Integer|Min(Integer) (+ (Variables|Default|GetSideOfRoad) 2) 1)))
  (:Canceled
    (Variables|Default|SetSideOfRoad (Math|Integer|Min(Integer) (Variables|Default|GetSideOfRoad) 1) :!label _label))
  (:Completed
    (goto _label)))

(event Input|EnhancedActionEvents|EnhancedInputActionIA_FWD
  (params (ActionValue :type Boolean) (ElapsedSeconds :type Float%20%28double-precision%29) (TriggeredSeconds :type Float%20%28double-precision%29) (InputAction :type Input%20Action%20Object%20Reference :default "/Game/Input/Test/IA_FWD.IA_FWD"))
  ;[1 1 1] Throttle
  (:Triggered
    (Class|ChaosVehicleMovementComponent|SetThrottleInput (Variables|Default|GetVehicleMovementComponent) 1.0))
  (:Canceled
    (Class|ChaosVehicleMovementComponent|SetThrottleInput (Variables|Default|GetVehicleMovementComponent) 0.0 :!label _label))
  (:Completed
    (goto _label)))

(event EventBeginPlay
  (|CallParentFunction))

(event Collision|EventActorBeginOverlap
  (params (OtherActor :type Actor%20Object%20Reference)))

(event EventTick
  (params (DeltaSeconds :type Float%20%28single-precision%29))
  (|CallParentFunction DeltaSeconds))

(event Input|KeyboardEvents|DebugKeyTab
  (params (Key :type Key%20Structure :default "None") (ActionValue :type Input%20Action%20Value%20Structure))
  (bind _returnvalue (Game|GetGameInstance))
  (:Pressed
    (Class|BPISaveGame|LoadSlots(Message) _returnvalue false)
    (bind _slots (Class|BPISaveGame|GetSlotsData(Message) _returnvalue))
    (for _array_element (Variables|/Game/Saves/BP_Slots.BP_Slots_C|GetSlotNames _slots)
      (Development|PrintString _array_element))))

(event Input|KeyboardEvents|DebugKeyT
  (params (Key :type Key%20Structure :default "None") (ActionValue :type Input%20Action%20Value%20Structure))
  ;[1 1 1] Debug
  (:Pressed
    (bind _returnvalue (UserInterface|CreateWidget "/Game/UI/Menus/LevelSelection/WB_LevelSelection.WB_LevelSelection_C" (Game|GetPlayerController 0)))
    (UserInterface|Viewport|AddtoViewport _returnvalue 0)))

(event Input|KeyboardEvents|DebugKeyH
  (params (Key :type Key%20Structure :default "None") (ActionValue :type Input%20Action%20Value%20Structure))
  ;[1 1 1] Debug
  (:Pressed
    (bind _savegamedata (Class|BPISaveGame|GetGameData(Message) (Game|GetGameInstance)))
    (Development|PrintString (Utilities|String|ToString(Integer) (Variables|/Game/Saves/BP_SaveGame.BP_SaveGame_C|GetLastPlayedLevelIndex _savegamedata)))
    (CallFunction|OpenLastPlayedLevel)))

(fn ConstructionScript
  (|CallParentFunction))