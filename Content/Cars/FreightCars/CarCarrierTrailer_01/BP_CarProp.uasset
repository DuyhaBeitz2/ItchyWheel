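; BP_CarProp is a physics-driven vehicle prop that reacts to hits, filed under the car carrier trailer assets.
; Until bumped, each hit sets physics simulation from CanBeActive and applies throttle; with BumpsOnHit, hard impacts launch it upward and randomly sideways, then spin it after a short delay.
; Once bumped, the first hit from anything except the player pawn restarts physics simulation.
; Drive applies throttle and releases the handbrake, while Stop is empty.
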(event Custom|Stop)

(event Custom|Drive
  (Class|ChaosVehicleMovementComponent|SetThrottleInput (Variables|Default|GetVehicleMovementComponent) (Variables|Default|GetThottle))
  (Class|ChaosVehicleMovementComponent|SetHandbrakeInput (Variables|Default|GetVehicleMovementComponent) false))

(event EventBeginPlay
  (|CallParentFunction) ; This node is disabled and will not be called.\nDrag off pins to build functionality.
)

(event Collision|EventActorBeginOverlap
  (params (OtherActor :type Actor%20Object%20Reference)))

(event EventTick
  (params (DeltaSeconds :type Float%20%28single-precision%29))
  (|CallParentFunction DeltaSeconds) ; This node is disabled and will not be called.\nDrag off pins to build functionality.
)

(event Collision|EventHit
  (params (MyComp :type Primitive%20Component%20Object%20Reference) (Other :type Actor%20Object%20Reference) (OtherComp :type Primitive%20Component%20Object%20Reference) (bSelfMoved :type Boolean) (HitLocation :type Vector :default "0, 0, 0") (HitNormal :type Vector :default "0, 0, 0") (NormalImpulse :type Vector :default "0, 0, 0") (Hit :type Hit%20Result%20Structure%20%28by%20ref%29))
  (bind _mesh (Variables|Character|GetMesh))
  (if (Variables|Default|GetBumped)
    (if (and (!= Other (Game|Player|GetPlayerPawn 0)) (not (Variables|Default|GetHasSwitchePhysics)))
      (Physics|SetSimulatePhysics (Variables|Character|GetMesh) false)
      (Physics|SetSimulatePhysics (Variables|Character|GetMesh) true)
      (Variables|Default|SetHasSwitchePhysics true))
    (else
      (Physics|SetSimulatePhysics (Variables|Character|GetMesh) (Variables|Default|GetCanBeActive))
      (Class|ChaosVehicleMovementComponent|SetThrottleInput (Variables|Default|GetVehicleMovementComponent) (Variables|Default|GetThottle))
      (if (and (> (Math|Vector|VectorLength NormalImpulse) 2e+04) (Variables|Default|GetBumpsOnHit))
        (Physics|AddImpulse _mesh (* (+ (Transformation|GetActorUpVector) (* (Transformation|GetActorRightVector) (Math|Integer|SelectInt 1 -1 (Math|Random|RandomBool)))) 6e+02) "Root" true)
        (Utilities|FlowControl|Delay 0.02)
        (Class|PrimitiveComponent|AddAngularImpulseinDegrees _mesh (Math|Vector|MakeVectorNetQuantize 1.8e+02 0.0 0.0) "Root" true)
        (Variables|Default|SetBumped true)))))

(fn ConstructionScript
  (|CallParentFunction))