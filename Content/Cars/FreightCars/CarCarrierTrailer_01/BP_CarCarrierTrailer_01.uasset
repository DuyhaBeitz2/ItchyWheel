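; Car carrier trailer with a moving lift, which attaches to a BP_CarCarrierTruck through a physics constraint on dock overlap.
; Tick moves the lift while the player pawn occupies its box, stops it otherwise, and flips direction at either end.
; A return-checker overlap sends a raised lift back down.
; The IMC area notifies BP_Test actors on entry and exit, passing the trailer and its child-actor path on entry.
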(event OnComponentBeginOverlap(Box)
  (params (OverlappedComponent :type Primitive%20Component%20Object%20Reference) (OtherActor :type Actor%20Object%20Reference) (OtherComp :type Primitive%20Component%20Object%20Reference) (OtherBodyIndex :type Integer) (bFromSweep :type Boolean) (SweepResult :type Hit%20Result%20Structure%20%28by%20ref%29))
  (if (== OtherActor (Game|Player|GetPlayerPawn 0))
    (Variables|Default|SetLiftActive true)))

(event OnComponentBeginOverlap(BoxIMCArea)
  (params (OverlappedComponent :type Primitive%20Component%20Object%20Reference) (OtherActor :type Actor%20Object%20Reference) (OtherComp :type Primitive%20Component%20Object%20Reference) (OtherBodyIndex :type Integer) (bFromSweep :type Boolean) (SweepResult :type Hit%20Result%20Structure%20%28by%20ref%29))
  (bind _asbp_test (Utilities|Casting|CastToBP_Test OtherActor))
  (bind _asbp_path (Utilities|Casting|CastToBP_Path (Variables|/Script/Engine.ChildActorComponent|GetChildActor (Variables|Default|GetPath_0))))
  (Default|EnteredCarCarrier _asbp_test _asbp_path self false))

(event OnComponentEndOverlap(BoxIMCArea)
  (params (OverlappedComponent :type Primitive%20Component%20Object%20Reference) (OtherActor :type Actor%20Object%20Reference) (OtherComp :type Primitive%20Component%20Object%20Reference) (OtherBodyIndex :type Integer))
  (bind _asbp_test (Utilities|Casting|CastToBP_Test OtherActor))
  (Default|LefttheCarCarrier _asbp_test))

(event OnComponentBeginOverlap(BoxDock)
  (params (OverlappedComponent :type Primitive%20Component%20Object%20Reference) (OtherActor :type Actor%20Object%20Reference) (OtherComp :type Primitive%20Component%20Object%20Reference) (OtherBodyIndex :type Integer) (bFromSweep :type Boolean) (SweepResult :type Hit%20Result%20Structure%20%28by%20ref%29))
  (bind _asbp_car_carrier_truck (Utilities|Casting|CastToBP_CarCarrierTruck OtherActor))
  (Class|PhysicsConstraintComponent|SetConstrainedComponents (Variables|Default|GetPhysicsConstraint) (Variables|/Script/ChaosVehicles.WheeledVehiclePawn|GetMesh _asbp_car_carrier_truck) "Root" (Variables|Character|GetMesh) "Root"))

(event OnComponentEndOverlap(Box)
  (params (OverlappedComponent :type Primitive%20Component%20Object%20Reference) (OtherActor :type Actor%20Object%20Reference) (OtherComp :type Primitive%20Component%20Object%20Reference) (OtherBodyIndex :type Integer))
  (if (== OtherActor (Game|Player|GetPlayerPawn 0))
    (Variables|Default|SetLiftActive false)))

(event OnComponentBeginOverlap(BoxReturnChecker)
  (params (OverlappedComponent :type Primitive%20Component%20Object%20Reference) (OtherActor :type Actor%20Object%20Reference) (OtherComp :type Primitive%20Component%20Object%20Reference) (OtherBodyIndex :type Integer) (bFromSweep :type Boolean) (SweepResult :type Hit%20Result%20Structure%20%28by%20ref%29))
  (if (not (Variables|Default|GetonBottom))
    (Variables|Default|SetLiftActive true)
    (Variables|Default|SetDirection false)))

(event OnComponentEndOverlap(BoxReturnChecker)
  (params (OverlappedComponent :type Primitive%20Component%20Object%20Reference) (OtherActor :type Actor%20Object%20Reference) (OtherComp :type Primitive%20Component%20Object%20Reference) (OtherBodyIndex :type Integer))
  (Variables|Default|SetLiftActive false))

(event EventTick
  (params (DeltaSeconds :type Float%20%28single-precision%29))
  (Utilities|FlowControl|Sequence
    (:then_0
      ;[1 1 1] Lift movement
      (if (Variables|Default|GetLiftActive)
        (Utilities|FlowControl|DoOnce false :!label _label
          (:Completed
            (Components|MoveComponentTo (Variables|Default|GetCarCarrierTrailer_01_LIFT) (Math|Vector|SelectVector (Variables|/Script/Engine.SceneComponent|GetRelativeLocation (Variables|Default|GetLiftTop)) (Variables|Default|GetInitialLiftLocation) (Variables|Default|GetDirection)) "0, 0, 0" false false 2.0 false :!label _label_2)))
        (else
          (Utilities|FlowControl|Sequence
            (:then_0
              (goto _label Reset))
            (:then_1
              (goto _label_2 Stop))))))
    (:then_1
      ;[1 1 1] Lift top/bottom positions
      (bind _output_get (Variables|Default|SetOnTop (Utilities|Operators|EqualEqual (Variables|/Script/Engine.SceneComponent|GetRelativeLocation (Variables|Default|GetCarCarrierTrailer_01_LIFT)) (Variables|/Script/Engine.SceneComponent|GetRelativeLocation (Variables|Default|GetLiftTop)) 0.0001)))
      (bind _output_get_2 (Variables|Default|SetonBottom (Utilities|Operators|EqualEqual (Variables|/Script/Engine.SceneComponent|GetRelativeLocation (Variables|Default|GetCarCarrierTrailer_01_LIFT)) (Variables|Default|GetInitialLiftLocation) 0.0001)))
      (if (or _output_get_2 _output_get)
        (Utilities|FlowControl|DoOnce false :!label _label_3
          (:Completed
            (Variables|Default|SetDirection (not (Variables|Default|GetDirection)))))
        (else
          (goto _label_3 Reset))))))

(fn ConstructionScript
  (Variables|Default|SetInitialLiftLocation (Variables|/Script/Engine.SceneComponent|GetRelativeLocation (Variables|Default|GetCarCarrierTrailer_01_LIFT))))