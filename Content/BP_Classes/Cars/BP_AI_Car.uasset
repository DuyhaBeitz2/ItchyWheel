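; AI-driven car that follows a BP_Path spline, picked by index or proximity, or drives toward goal actors until the final one is reached.
; Each tick it steers at a look-ahead point or the goal and sets throttle from a curve of upcoming turn angle, pulsing the handbrake in fast turns.
; A speed-scaled forward sphere trace for vehicles triggers handbrake stops, as does a temporary forced slowdown.
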(event Custom|CheckForObstacles
  (bind _arrow (Variables|Default|GetArrow))
  (bind _returnvalue (Transformation|GetWorldLocation _arrow))
  ;[1 1 1] Check for obstacles
  (bind (_outhit _returnvalue_2) (Collision|SphereTraceForObjects _returnvalue (+ _returnvalue (* (Transformation|GetActorForwardVector) (Math|Float|Min(Float) (+ (Variables|Default|GetInitialLineLength) (Math|Float|Square (Class|ChaosVehicleMovementComponent|GetForwardSpeedMPH (Variables|Default|GetVehicleMovementComponent)))) 3.5e+02))) 8e+01 (Utilities|Array|MakeArray (Utilities|Enum|LiteralenumEObjectTypeQuery "ObjectTypeQuery5")) false (Utilities|Array|MakeArray self) "None"))
  (if _returnvalue_2
    (if (or (> (Math|Vector|VectorLength (- (Transformation|GetVelocity (.HitActor (Collision|BreakHitResult _outhit))) (Transformation|GetVelocity))) 6e+01) (< (Math|Vector|VectorLength (- (Transformation|GetActorLocation (.HitActor (Collision|BreakHitResult _outhit))) (Transformation|GetActorLocation))) 1e+02))
      (Variables|CarDefault|SetStanding true)
      (else
        (Variables|CarDefault|SetStanding false :!label _label)))
    (else
      (goto _label))))

(event Custom|AutomaticallyAccelerate
  ;[1 1 1] Automatically accelerate
  (bind _angle (CallFunction|AngleOfTurn (Variables|Default|GetPath) 1.2e+03 (Variables|Default|GetGoal) (Variables|CarDefault|GetFollowSpline)))
  (Class|ChaosVehicleMovementComponent|SetThrottleInput (Variables|Default|GetVehicleMovementComponent) (Math|Curves|GetFloatValue (Variables|Default|GetThrottleCurve) (Math|Float|Absolute(Float) _angle)))
  (Variables|Default|SetWasTurning (> (Math|Float|Absolute(Float) _angle) 7.0))
  (if (and (> (Math|Float|Absolute(Float) _angle) 7.0) (> (Class|ChaosVehicleMovementComponent|GetForwardSpeedMPH (Variables|Default|GetVehicleMovementComponent)) 15.0))
    (Class|ChaosVehicleMovementComponent|SetHandbrakeInput (Variables|Default|GetVehicleMovementComponent) true)
    (Utilities|FlowControl|Delay 0.2)
    (Class|ChaosVehicleMovementComponent|SetHandbrakeInput (Variables|Default|GetVehicleMovementComponent) false)
    (Utilities|FlowControl|Delay 0.2)
    (Variables|Default|SetWasTurning false)
    (else
      (Variables|CarDefault|SetStanding false))))

(event Custom|GoalReached
  (params (NextGoal :type BP%20AI%20Goal%20Object%20Reference) (ItWasFinalGoal :type Boolean))
  (if ItWasFinalGoal
    (Variables|Default|SetAI_Active false)
    (else
      (Variables|Default|SetGoal NextGoal))))

(event Custom|ForceSlowDown
  (if (> (Class|ChaosVehicleMovementComponent|GetForwardSpeedMPH (Variables|Default|GetVehicleMovementComponent)) 5.0)
    (Variables|Default|SetForceSlowDown? true)
    (Utilities|FlowControl|Delay 0.5)
    (Variables|Default|SetForceSlowDown? false)))

(event EventBeginPlay
  (Class|ChaosVehicleMovementComponent|SetThrottleInput (Variables|Default|GetVehicleMovementComponent) (Variables|CarDefault|GetDefaultThrottle))
  (bind _outactors (Actor|GetAllActorsOfClass "/Game/BP_Classes/BP_Path.BP_Path_C"))
  (bind _closestpath (CallFunction|GetCarPath (Variables|CarDefault|GetPathIndex) _outactors))
  (Variables|Default|SetPath _closestpath))

(event EventTick
  (params (DeltaSeconds :type Float%20%28single-precision%29))
  (bind _vehiclemovementcomponent (Variables|Default|GetVehicleMovementComponent))
  (if (Variables|Default|GetAI_Active)
    (if (Variables|Default|GetForceSlowDown?)
      (Class|ChaosVehicleMovementComponent|SetHandbrakeInput (Variables|Default|GetVehicleMovementComponent) true)
      (else
        (CallFunction|CheckforObstacles)
        (if (not (Variables|CarDefault|GetStanding))
          (Class|ChaosVehicleMovementComponent|SetHandbrakeInput _vehiclemovementcomponent false)
          (if (Variables|CarDefault|GetFollowSpline)
            (Utilities|FlowControl|Sequence
              (:then_0
                (bind _steering (CallFunction|GetSteeringfromPath (Variables|Default|GetPath) 5e+02))
                (Class|ChaosVehicleMovementComponent|SetSteeringInput (Variables|Default|GetVehicleMovementComponent) _steering))
              (:then_1
                (CallFunction|AutomaticallyAccelerate)
                (CallFunction|FindSteeringto (Transformation|GetActorLocation) (Transformation|GetActorLocation (Variables|Default|GetGoal)))))
            (else
              (bind _steering_2 (CallFunction|FindSteeringto (Transformation|GetActorLocation) (Transformation|GetActorLocation (Variables|Default|GetGoal))))
              (Class|ChaosVehicleMovementComponent|SetSteeringInput (Variables|Default|GetVehicleMovementComponent) _steering_2)
              (CallFunction|AutomaticallyAccelerate)))
          (else
            (Class|ChaosVehicleMovementComponent|SetHandbrakeInput _vehiclemovementcomponent true :!label _label)))))
    (else
      (goto _label))))

(fn ConstructionScript)

(fn GetSteeringfromPath
  (params (Path :type BP%20Path%20Object%20Reference) (DistanceAhead :type Float%20%28double-precision%29))
  (bind _returnvalue (Transformation|GetActorLocation))
  (bind _spline (Variables|/Game/BP_Classes/BP_Path.BP_Path_C|GetSpline Path))
  (bind _returnvalue_2 (Class|SplineComponent|FindTangentClosesttoWorldLocation _spline _returnvalue "World"))
  (bind _returnvalue_3 (Math|Vector|Normalize _returnvalue_2))
  (bind _returnvalue_4 (* _returnvalue_3 DistanceAhead))
  (bind _returnvalue_5 (+ _returnvalue_4 _returnvalue))
  (bind _returnvalue_6 (Spline|FindLocationClosesttoWorldLocation _spline _returnvalue_5 "World"))
  (Rendering|Debug|DrawDebugSphere _returnvalue_6 25.0 12 "(R=0.000000,G=0.000000,B=0.000000,A=1.000000)" 0.0)
  (bind _steering (CallFunction|FindSteeringto _returnvalue _returnvalue_6))
  (return _steering))

(fn FindSteeringto
  (params (From :type Vector) (To :type Vector))
  (return (Math|Float|MapRangeClamped (.Yaw (Math|Rotator|BreakRotator (Math|Rotator|Delta(Rotator) (Math|Rotator|FindLookatRotation From To) (Transformation|GetActorRotation)))) -25.0 25.0 -1.0 1.0)))

(fn AngleOfTurn
  (params (Path :type BP%20Path%20Object%20Reference) (DistanceAhead :type Float%20%28double-precision%29) (Goal :type BP%20AI%20Goal%20Object%20Reference) (ChoosePathInsteadOfGoal :type Boolean))
  (bind _returnvalue (Transformation|GetActorLocation))
  (bind _spline (Variables|/Game/BP_Classes/BP_Path.BP_Path_C|GetSpline Path))
  (if ChoosePathInsteadOfGoal
    (bind _yaw (CallFunction|FindAngletoPos (Class|SplineComponent|FindTangentClosesttoWorldLocation _spline (+ (* (Math|Vector|Normalize (Class|SplineComponent|FindTangentClosesttoWorldLocation _spline _returnvalue "World")) DistanceAhead) _returnvalue) "World")))
    (return _yaw)
    (else
      (bind _yaw_2 (CallFunction|FindAngletoPos (Transformation|GetActorLocation (Variables|Default|GetGoal))))
      (return _yaw_2))))

(fn GetCarPath
  (params (Index :type Integer) (Paths :type Array%20of%20BP%20Path%20Object%20References))
  (if (Variables|CarDefault|GetTakeClosestPath)
    (for _array_element Paths
      (LocalVariables|SetMinDistance (Math|Float|Min(Float) (LocalVariables|GetMinDistance) (Math|Vector|Distance(Vector) (Transformation|GetActorLocation _array_element) (Transformation|GetActorLocation))))
      (if (== (Math|Vector|Distance(Vector) (Transformation|GetActorLocation _array_element) (Transformation|GetActorLocation)) (LocalVariables|GetMinDistance))
        (LocalVariables|SetPathClosest _array_element)))
    (return (LocalVariables|GetPathClosest))
    (else
      (return (Utilities|Array|Get(acopy) Paths Index)))))

(fn FindAngletoPos
  (params (TargetLocation :type Vector))
  (bind _returnvalue (Transformation|GetActorLocation))
  (return (.Yaw (Math|Rotator|BreakRotator (Math|Rotator|Delta(Rotator) (Math|Rotator|FindLookatRotation _returnvalue (+ _returnvalue TargetLocation)) (Transformation|GetActorRotation))))))