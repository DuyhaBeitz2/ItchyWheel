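; AI-driven vehicle that follows a BP_Path spline on one side of the road, or shadows a target actor.
; Each tick steers toward a speed-scaled look-ahead point, adjusted for turns, and sets throttle, brake and handbrake from path curvature.
; Overlap boxes, the front one shifting with speed, drive overtaking by side-switching or speed capping; vehicle hits can also switch sides.
; Material parameters drive brake and turn lights.
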(event OnComponentHit(Mesh)
  (params (HitComponent :type Primitive%20Component%20Object%20Reference) (OtherActor :type Actor%20Object%20Reference) (OtherComp :type Primitive%20Component%20Object%20Reference) (NormalImpulse :type Vector :default "0, 0, 0") (Hit :type Hit%20Result%20Structure%20%28by%20ref%29))
  ;[1 1 1] Switch side of road if its already taken
  (bind _asbp_vehicle_ai (Utilities|Casting|CastToBP_VehicleAI OtherActor))
  (if (> (Variables|Road|GetSideOfRoad) 0)
    (Utilities|FlowControl|Sequence
      (:then_0
        (if (< (Math|Vector|Distance(Vector) (Transformation|GetActorLocation _asbp_vehicle_ai) (+ (Transformation|GetActorLocation) (* (Transformation|GetActorRightVector) 1e+02))) 1e+02)
          (Variables|Road|SetSideOfRoad -1))))
    (elif (< (Math|Vector|Distance(Vector) (Transformation|GetActorLocation _asbp_vehicle_ai) (+ (Transformation|GetActorLocation) (* (Transformation|GetActorRightVector) -1e+02))) 1e+02)
      (Variables|Road|SetSideOfRoad 1))))

(event EventBeginPlay
  (Utilities|FlowControl|Sequence
    (:then_0
      (if (Variables|Road|GetAutomaticallySelectClosestPath)
        (bind _path (CallFunction|GetClosestPath))
        (bind _output_get (Variables|Road|SetPath _path))
        (Variables|Default|SetPathSpline (Variables|/Game/BP_Classes/BP_Path.BP_Path_C|GetSpline _output_get))))
    (:then_1
      (if (Variables|Road|GetAutomaticallySelectSideOfRoadOnStart)
        (bind _closestsideofroad (CallFunction|CalculateClosestSideOfRoad))
        (Variables|Road|SetSideOfRoad _closestsideofroad)))))

(event EventTick
  (params (DeltaSeconds :type Float%20%28single-precision%29))
  (bind _target (Variables|Follow|GetTarget))
  (bind _initailboxlocation (Variables|Default|GetInitailBoxLocation))
  (bind _returnvalue (Transformation|GetActorLocation _target))
  (bind (_x _y _z) (Math|Vector|BreakVector _initailboxlocation))
  (CallFunction|UpdateLights)
  (if (Variables|Default|GetStopOverride)
    (Class|ChaosVehicleMovementComponent|SetHandbrakeInput (Variables|Default|GetVehicleMovementComponent) true)
    (else
      (Utilities|FlowControl|Sequence
        (:then_0
          (CallFunction|CollisionsandOvertakes)
          ;[1 1 1] Steering
          (if (Variables|AI|GetAIControlSteering)
            (bind _steering (CallFunction|CalculateSteering))
            (Class|ChaosVehicleMovementComponent|SetSteeringInput (Variables|Default|GetVehicleMovementComponent) _steering)
            ;[1 1 1] Adjust steering depending on inside/outside turn
            (bind (_turningoninsideloop _turningonoutsideloop) (CallFunction|TurningontheInsideorOutsideLoop))
            (Variables|Default|SetOverrideMaxTurningDistance? false)
            (if _turningoninsideloop
              (Variables|Default|SetOverrideMaxTurningDistance? true)
              (Variables|Default|SetOverrideMaxTurningDistance (+ (Variables|Steering|GetMaxTurningDistanceAhead) 4e+02))
              (Variables|Default|SetOverrideMinTurningDistance? true)
              (Variables|Default|SetOverrideMinTurningDistance (+ (Variables|Steering|GetMinTurningDistanceAhead) 5e+01))
              (elif _turningonoutsideloop
                (Variables|Default|SetOverrideMaxTurningDistance? true)
                (Variables|Default|SetOverrideMaxTurningDistance (- (Variables|Steering|GetMaxTurningDistanceAhead) 7e+02))
                (Variables|Default|SetOverrideMinTurningDistance? true)
                (Variables|Default|SetOverrideMinTurningDistance (Math|Float|Max(Float) (- (Variables|Steering|GetMinTurningDistanceAhead) 3e+02) 0.0))))))
        (:then_1
          ;[1 1 1] Throttle/Brake
          (if (Variables|AI|GetAIControlThrottle/brake/handbrake)
            (bind _topspeed (CallFunction|CalculateTopSpeed))
            (bind (_throttle _brake _handbrake) (CallFunction|CalculateThrottle/brake/handbrake _topspeed))
            (Class|ChaosVehicleMovementComponent|SetThrottleInput (Variables|Default|GetVehicleMovementComponent) _throttle)
            (Class|ChaosVehicleMovementComponent|SetBrakeInput (Variables|Default|GetVehicleMovementComponent) _brake)
            (Class|ChaosVehicleMovementComponent|SetHandbrakeInput (Variables|Default|GetVehicleMovementComponent) _handbrake)))
        (:then_2
          ;[1 1 1] Adjust front box depending on speed
          (bind _returnvalue_2 (CallFunction|GetKmPerH))
          (Transformation|SetRelativeLocation (Variables|Default|GetFrontBox) (Math|Vector|MakeVector (+ _x (Math|Float|MapRangeClamped _returnvalue_2 (Variables|Speed|GetMinSpeed%28calc%29) (Variables|Speed|GetMaxSpeed%28calc%29) 0.0 (Variables|Default|GetMaxBoxOffset))) _y _z) false false))
        (:then_3
          ;[1 1 1] Choose path to follow target
          (if (Variables|Follow|GetFollowTarget)
            (bind _asbp_vehicle_ai (Utilities|Casting|CastToBP_VehicleAI (Variables|Follow|GetTarget)))
            (bind _output_get (Variables|Road|SetPath (Variables|BP_VehicleAI_C|GetPath _asbp_vehicle_ai)))
            (Variables|Default|SetPathSpline (Variables|/Game/BP_Classes/BP_Path.BP_Path_C|GetSpline _output_get))
            ;[1 1 1] Steer directly to target
            (if (Variables|Follow|GetSteerDirectlyToTarget%28dynamic%29)
              (if (Variables|Follow|GetAvoidCollidingWithTarget)
                (bind _steering_2 (CallFunction|CalculateSteeringtoLocation (+ (* (Transformation|GetActorForwardVector _target) -500) _returnvalue)))
                (Class|ChaosVehicleMovementComponent|SetSteeringInput (Variables|Default|GetVehicleMovementComponent) _steering_2)
                (else
                  (bind _steering_3 (CallFunction|CalculateSteeringtoLocation _returnvalue))
                  (Class|ChaosVehicleMovementComponent|SetSteeringInput (Variables|Default|GetVehicleMovementComponent) _steering_3))))))))))

(fn ConstructionScript
  (Variables|Default|SetInitailBoxLocation (Variables|/Script/Engine.SceneComponent|GetRelativeLocation (Variables|Default|GetFrontBox)))
  (Rendering|SetVisibility (Variables|Default|GetSpotLight1) (Variables|Default|GetLightsOn) false)
  (Rendering|SetVisibility (Variables|Default|GetSpotLight) (Variables|Default|GetLightsOn) false)
  (Rendering|Material|SetScalarParameterValueonMaterials (Variables|Character|GetMesh) "FrontLightsIntensity" (Math|Conversions|ToFloat(Boolean) (Variables|Default|GetLightsOn))))

(fn GetKmPerH
  (return (* (Vehicle|GetForwardSpeed (Variables|Default|GetVehicleMovementComponent)) 0.036)))

(fn CalculateSteering
  (bind _returnvalue (CallFunction|GetKmPerH))
  (if (< _returnvalue -5.0)
    (return 0.0)
    (else
      ;[1 1 1] Find point to steer to
      (bind _returnvalue_2 (CallFunction|GetKmPerH))
      (bind _frontlocation (CallFunction|GetFrontWorldLocation))
      (bind _pointlocation (Default|GetClosestLocationtoAIPath (Variables|Road|GetPath) (Math|Float|MapRangeClamped _returnvalue_2 (Variables|Speed|GetMinSpeed%28calc%29) (Variables|Speed|GetMaxSpeed%28calc%29) (select (Variables|Default|GetOverrideMinTurningDistance?) (Variables|Default|GetOverrideMinTurningDistance) (Variables|Steering|GetMinTurningDistanceAhead)) (select (Variables|Default|GetOverrideMaxTurningDistance?) (Variables|Default|GetOverrideMaxTurningDistance) (Variables|Steering|GetMaxTurningDistanceAhead))) _frontlocation (Variables|Road|GetSideOfRoad)))
      (bind _steering (CallFunction|CalculateSteeringtoLocation _pointlocation))
      (return _steering))))

(fn GetClosestPath
  (bind _outactors (Actor|GetAllActorsOfClass "/Game/BP_Classes/BP_Path.BP_Path_C"))
  (for _array_element _outactors
    ;[1 1 1] Check if path is detectable
    (if (Variables|/Game/BP_Classes/BP_Path.BP_Path_C|GetDetectableOnStart _array_element)
      (bind _output_get (LocalVariables|SetCurrentArrayElementPath _array_element))
      ;[1 1 1] Distance to path
      (LocalVariables|SetDistance (Math|Vector|Distance(Vector) (Transformation|GetActorLocation _output_get) (Transformation|GetActorLocation)))
      (if (== (LocalVariables|GetMinDistance) -1.0)
        ;[1 1 1] Initial distance
        (LocalVariables|SetMinDistance (LocalVariables|GetDistance))
        (else
          ;[1 1 1] Min distance
          (LocalVariables|SetMinDistance (Math|Float|Min(Float) (LocalVariables|GetDistance) (LocalVariables|GetMinDistance)))))
      (if (== (LocalVariables|GetDistance) (LocalVariables|GetMinDistance))
        (LocalVariables|SetClosestPath (LocalVariables|GetCurrentArrayElementPath)))))
  ;[1 1 1] Return path
  (return (LocalVariables|GetClosestPath)))

(fn CalculateTopSpeed
  (if (Variables|Default|GetOverrideTopSpeed?)
    (return (Variables|Default|GetOverrideTopSpeed))
    (else
      ;[1 1 1] Find point to steer to
      (bind _returnvalue (CallFunction|GetKmPerH))
      (bind _frontlocation (CallFunction|GetFrontWorldLocation))
      (bind _pointlocation (Default|GetClosestLocationtoAIPath (Variables|Road|GetPath) (Math|Float|MapRangeClamped _returnvalue 5e+01 1.5e+02 3e+03 9e+03) _frontlocation (Variables|Road|GetSideOfRoad)))
      ;[1 1 1] Angle to point
      (bind _frontlocation_2 (CallFunction|GetFrontWorldLocation))
      (return (Math|Float|MapRangeClamped (Math|Float|Absolute(Float) (.Yaw (Math|Rotator|BreakRotator (Math|Rotator|Delta(Rotator) (Math|Rotator|FindLookatRotation _frontlocation_2 _pointlocation) (Transformation|GetActorRotation))))) 0.0 4e+01 (Variables|Speed|GetMaxSpeed%28calc%29) (Variables|Speed|GetMinSpeed%28calc%29))))))

(fn CalculateThrottle/brake/handbrake
  (params (TopSpeed :type Float%20%28double-precision%29))
  (bind _returnvalue (CallFunction|GetKmPerH))
  (if (>= _returnvalue TopSpeed)
    (if (> (- _returnvalue TopSpeed) 6.0)
      (return 0.0 1.0 true)
      (else
        (return 0.0 1.0 false)))
    (else
      (return 0.76 0.0 false))))

(fn GetFrontWorldLocation
  (return (Transformation|GetWorldLocation (Variables|Default|GetFrontArrow))))

(fn TurningontheInsideorOutsideLoop
  (bind _steering (CallFunction|CalculateSteering))
  (if (> _steering 0.2)
    (return (> (* (Variables|Road|GetSideOfRoad) _steering) 0.0) (< (* (Variables|Road|GetSideOfRoad) _steering) 0.0))
    (else
      (return false false))))

(fn CalculateClosestSideOfRoad
  (bind _returnvalue (Transformation|GetActorLocation))
  (bind _returnvalue_2 (Transformation|GetActorLocation))
  ;[1 1 1] Left side distance
  (bind _pointlocation (Default|GetClosestLocationtoAIPath (Variables|Road|GetPath) 0.0 _returnvalue_2 -1))
  (LocalVariables|SetleftSideDistance (Math|Vector|Distance(Vector) _pointlocation _returnvalue_2))
  ;[1 1 1] Right side distance
  (bind _pointlocation_2 (Default|GetClosestLocationtoAIPath (Variables|Road|GetPath) 0.0 _returnvalue 1))
  (LocalVariables|SetRightSideDistance (Math|Vector|Distance(Vector) _pointlocation_2 _returnvalue))
  (if (< (LocalVariables|GetleftSideDistance) (LocalVariables|GetRightSideDistance))
    (return -1)
    (else
      (return 1))))

(fn CollisionsandOvertakes
  (bind _frontbox (Variables|Default|GetFrontBox))
  (bind _overlappingactors (Collision|GetOverlappingActors _frontbox 0 :!class /Script/Engine.PrimitiveComponent))
  (Utilities|FlowControl|Sequence
    (:then_0
      ;[1 1 1] Is there vehicle in front?
      (bind _output_get (LocalVariables|SetVehicleInFront? (> (Utilities|Array|Length _overlappingactors) 0)))
      (if _output_get
        ;[1 1 1] Get actor vehicle in front
        (LocalVariables|SetVehicleInFront (Utilities|Array|Get(acopy) _overlappingactors))
        (LocalVariables|SetVehiclePreventsFromOvertaking (or (> (Utilities|Array|Length (Collision|GetOverlappingActors (Variables|Default|GetLeftBox) 0 :!class /Script/Engine.PrimitiveComponent)) 0) (> (Utilities|Array|Length (Collision|GetOverlappingActors (Variables|Default|GetRightBox) 0 :!class /Script/Engine.PrimitiveComponent)) 0)))))
    (:then_1
      (if (Variables|Follow|GetAvoidCollidingWithTarget)
        (Variables|Default|SetOverrideTopSpeed? false :!label _label)
        (if (LocalVariables|GetVehicleInFront?)
          (if (LocalVariables|GetVehiclePreventsFromOvertaking)
            ;[1 1 1] Avoid colliding into vehicle in front
            (Utilities|Casting|CastToBP_VehicleAI (LocalVariables|GetVehicleInFront) :!label _label_2)
            (if (< (Math|Vector|Distance(Vector) (Transformation|GetActorLocation (LocalVariables|GetVehicleInFront)) (Transformation|GetActorLocation)) 3e+03)
              (bind _returnvalue (CallFunction|GetKmPerH))
              (Variables|Default|SetOverrideTopSpeed (Math|Float|Max(Float) (- (* _returnvalue (Math|Trig|Sin(Degrees) (.yaw (Math|Rotator|Delta(Rotator) (Transformation|GetActorRotation (LocalVariables|GetVehicleInFront)) (Transformation|GetActorRotation))))) 1.0) 0.0))
              (Variables|Default|SetOverrideTopSpeed? true))
            (elif (Variables|AI|GetOvertakes?)
              (bind _asbp_vehicle_ai (Utilities|Casting|CastToBP_VehicleAI (LocalVariables|GetVehicleInFront)))
              (if (== (Variables|BP_VehicleAI_C|GetSideOfRoad _asbp_vehicle_ai) (Variables|Road|GetSideOfRoad))
                ;[1 1 1] Overtake
                (Variables|Road|SetSideOfRoad (* (Variables|Road|GetSideOfRoad) -1)))
              (else
                (goto _label_2)))))
        (elif (or (!= (LocalVariables|GetVehicleInFront) (Variables|Follow|GetTarget)) (not (Variables|Follow|GetFollowTarget)))
          (goto _label))))))

(fn GetDistance(Location)AlongPath
  (LocalVariables|SetDistance (Class|SplineComponent|GetDistanceAlongSplineatLocation (Variables|Default|GetPathSpline) (Transformation|GetActorLocation) "World"))
  (while (> (LocalVariables|GetDistance) (Spline|GetSplineLength (Variables|Default|GetPathSpline)))
    (LocalVariables|SetDistance 0.0))
  (return (LocalVariables|GetDistance)))

(fn CalculateSteeringtoLocation
  (params (Location :type Vector))
  (bind _steeringaccuracy (Variables|Steering|GetSteeringAccuracy))
  ;[1 1 1] Angle to point
  (bind _frontlocation (CallFunction|GetFrontWorldLocation))
  (return (Math|Float|MapRangeClamped (.Yaw (Math|Rotator|BreakRotator (Math|Rotator|Delta(Rotator) (Math|Rotator|FindLookatRotation _frontlocation Location) (Transformation|GetActorRotation)))) (* _steeringaccuracy -1.0) _steeringaccuracy -1.0 1.0)))

(fn UpdateLights
  (bind _vehiclemovementcomponent (Variables|Default|GetVehicleMovementComponent))
  (Rendering|Material|SetScalarParameterValueonMaterials (Variables|Character|GetMesh) "BreakLightsIntensity" (* (Math|Conversions|ToFloat(Boolean) (or (Class|ChaosVehicleMovementComponent|GetHandbrakeInput _vehiclemovementcomponent) (Class|ChaosVehicleMovementComponent|GetHandbrakeInput _vehiclemovementcomponent))) 2.0))
  (bind _returnvalue (Class|ChaosVehicleMovementComponent|GetSteeringInput (Variables|Default|GetVehicleMovementComponent)))
  (if (< _returnvalue -0.8)
    (Rendering|Material|SetScalarParameterValueonMaterials (Variables|Character|GetMesh) "LeftTurnLightsIntensity" 1.0)
    (else
      (Rendering|Material|SetScalarParameterValueonMaterials (Variables|Character|GetMesh) "LeftTurnLightsIntensity" 0.0)
      (if (> _returnvalue 0.8)
        (Rendering|Material|SetScalarParameterValueonMaterials (Variables|Character|GetMesh) "RightTurnLightsIntensity" 1.0)
        (else
          (Rendering|Material|SetScalarParameterValueonMaterials (Variables|Character|GetMesh) "RightTurnLightsIntensity" 0.0))))))