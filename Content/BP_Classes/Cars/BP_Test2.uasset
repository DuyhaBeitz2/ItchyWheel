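; Test car Blueprint, built on a path-aware vehicle parent, with player input for throttle, handbrake, camera look and road-side choice.
; Car carrier events zero the driving inputs, switch to the carrier's path with optional steering lock, and restore the closest path on leaving.
; Tick adds scaled trailer velocity to the car's movement component while aboard and holds steering at zero while locked.
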(event Custom|EnteredCarCarrier
  (params (Path :type BP%20Path%20Object%20Reference) (CarCarrier :type Wheeled%20Vehicle%20Pawn%20Object%20Reference) (LockSteering :type Boolean))
  (Variables|Default|SetSteeringLocked LockSteering)
  (Variables|Default|SetCarCarrier CarCarrier)
  (Variables|Default|SetCarCarrierPath Path)
  (Variables|Default|SetInCarCarrierTrailer true)
  (Class|ChaosVehicleMovementComponent|SetBrakeInput (Variables|Default|GetVehicleMovementComponent) 0.0)
  (Class|ChaosVehicleMovementComponent|SetThrottleInput (Variables|Default|GetVehicleMovementComponent) 0.0)
  (Class|ChaosVehicleMovementComponent|SetSteeringInput (Variables|Default|GetVehicleMovementComponent) 0.0)
  (bind _output_get (Variables|Default|SetPath (Variables|Default|GetCarCarrierPath)))
  (Variables|Default|SetPathSpline (Variables|/Game/BP_Classes/BP_Path.BP_Path_C|GetSpline _output_get)))

(event Custom|LeftTheCarCarrier
  (Variables|Default|SetInCarCarrierTrailer false)
  (Class|ChaosVehicleMovementComponent|SetBrakeInput (Variables|Default|GetVehicleMovementComponent) 0.0)
  (Class|ChaosVehicleMovementComponent|SetThrottleInput (Variables|Default|GetVehicleMovementComponent) 0.0)
  (bind _path (CallFunction|GetClosestPath))
  (bind _output_get (Variables|Default|SetPath _path))
  (Variables|Default|SetPathSpline (Variables|/Game/BP_Classes/BP_Path.BP_Path_C|GetSpline _output_get))
  (Variables|Default|SetSteeringLocked false))

(event Input|EnhancedActionEvents|EnhancedInputActionIA_LookAround
  (params (ActionValue :type Vector%202D%20Structure) (ElapsedSeconds :type Float%20%28double-precision%29) (TriggeredSeconds :type Float%20%28double-precision%29) (InputAction :type Input%20Action%20Object%20Reference :default "/Game/Input/Test/IA_LookAround.IA_LookAround"))
  (bind (_x _y) (Math|Vector2D|BreakVector2D ActionValue))
  ;[1 1 1] Look Around
  (Pawn|Input|AddControllerYawInput _x)
  (Pawn|Input|AddControllerPitchInput _y))

(event Input|EnhancedActionEvents|EnhancedInputActionIA_Handbrake
  (params (ActionValue :type Boolean) (ElapsedSeconds :type Float%20%28double-precision%29) (TriggeredSeconds :type Float%20%28double-precision%29) (InputAction :type Input%20Action%20Object%20Reference :default "/Game/Input/Test/IA_Handbrake.IA_Handbrake"))
  ;[1 1 1] Handbrake
  (:Triggered
    (Class|ChaosVehicleMovementComponent|SetHandbrakeInput (Variables|Default|GetVehicleMovementComponent) true))
  (:Canceled
    (Class|ChaosVehicleMovementComponent|SetHandbrakeInput (Variables|Default|GetVehicleMovementComponent) false :!label _label))
  (:Completed
    (goto _label)))

(event Input|EnhancedActionEvents|EnhancedInputActionIA_LeftSideOfRoad
  (params (ActionValue :type Boolean) (ElapsedSeconds :type Float%20%28double-precision%29) (TriggeredSeconds :type Float%20%28double-precision%29) (InputAction :type Input%20Action%20Object%20Reference :default "/Game/Input/Test/IA_LeftSideOfRoad.IA_LeftSideOfRoad"))
  (Variables|Default|SetSideOfRoad -1))

(event Input|EnhancedActionEvents|EnhancedInputActionIA_RightSideOfRoad
  (params (ActionValue :type Boolean) (ElapsedSeconds :type Float%20%28double-precision%29) (TriggeredSeconds :type Float%20%28double-precision%29) (InputAction :type Input%20Action%20Object%20Reference :default "/Game/Input/Test/IA_RightSideOfRoad.IA_RightSideOfRoad"))
  (Variables|Default|SetSideOfRoad 1))

(event Input|EnhancedActionEvents|EnhancedInputActionIA_FWD
  (params (ActionValue :type Boolean) (ElapsedSeconds :type Float%20%28double-precision%29) (TriggeredSeconds :type Float%20%28double-precision%29) (InputAction :type Input%20Action%20Object%20Reference :default "/Game/Input/Test/IA_FWD.IA_FWD"))
  ;[1 1 1] Throttle
  (:Triggered
    (Class|ChaosVehicleMovementComponent|SetThrottleInput (Variables|Default|GetVehicleMovementComponent) 1.0))
  (:Canceled
    (Class|ChaosVehicleMovementComponent|SetThrottleInput (Variables|Default|GetVehicleMovementComponent) 0.0 :!label _label))
  (:Completed
    (goto _label)))

(event EventBeginPlay
  ;[1 1 1] Add mapping context
  (|CallParentFunction)
  (bind _asplayer_controller (Utilities|Casting|CastToPlayerController (Pawn|GetController)))
  (Input|AddMappingContext (PlayerController|LocalPlayerSubsystems|GetEnhancedInputLocalPlayerSubsystem _asplayer_controller) "/Game/Input/Test/IMC_Test.IMC_Test" 0 "(bIgnoreAllPressedKeysUntilRelease=True,bForceImmediately=False,bNotifyUserSettings=False)"))

(event Collision|EventActorBeginOverlap
  (params (OtherActor :type Actor%20Object%20Reference)))

(event EventTick
  (params (DeltaSeconds :type Float%20%28single-precision%29))
  (bind _vehiclemovementcomponent (Variables|Default|GetVehicleMovementComponent))
  (|CallParentFunction DeltaSeconds)
  (Utilities|FlowControl|Sequence
    (:then_0
      (if (Variables|Default|GetInCarCarrierTrailer)
        (Utilities|Casting|CastToBP_CarCarrierTrailer_01 (Variables|Default|GetCarCarrier))
        (Variables|/Script/Engine.MovementComponent|SetVelocity _vehiclemovementcomponent (+ (Variables|/Script/Engine.MovementComponent|GetVelocity _vehiclemovementcomponent) (* (Variables|/Script/Engine.MovementComponent|GetVelocity (Variables|/Script/ChaosVehicles.WheeledVehiclePawn|GetVehicleMovementComponent (Variables|Default|GetCarCarrier))) 50)))))
    (:then_1
      (if (Variables|Default|GetSteeringLocked)
        (Class|ChaosVehicleMovementComponent|SetSteeringInput (Variables|Default|GetVehicleMovementComponent) 0.0)))))

(fn ConstructionScript
  (|CallParentFunction)
  (Variables|Default|SetInitialMaxDistanceAhead (Variables|Default|GetMaxTurningDistanceAhead))
  (Variables|Default|SetInitialMinTurningDistanceAhead (Variables|Default|GetMinTurningDistanceAhead)))