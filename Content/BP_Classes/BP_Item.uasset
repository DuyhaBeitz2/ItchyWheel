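; BP_Item is an item actor that optionally hovers and spins, and reacts when something overlaps its sphere.
; Tick accumulates time to drive a sine-based bob above the location cached in the construction script and a constant yaw rotation, each behind its own toggle.
; On overlap, optionally limited to the player pawn, the sphere ignores all further collision and can hide itself and its children.
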(event OnComponentBeginOverlap(Sphere)
  (params (OverlappedComponent :type Primitive%20Component%20Object%20Reference) (OtherActor :type Actor%20Object%20Reference) (OtherComp :type Primitive%20Component%20Object%20Reference) (OtherBodyIndex :type Integer) (bFromSweep :type Boolean) (SweepResult :type Hit%20Result%20Structure%20%28by%20ref%29))
  (if (or (== OtherActor (Game|Player|GetPlayerPawn 0)) (not (Variables|Default|GetOnlyForPlayer)))
    (Collision|SetCollisionResponsetoAllChannels (Variables|Default|GetSphere) "ECR_Ignore")
    (if (Variables|Default|GetHideOnOverlap)
      (Rendering|SetVisibility (Variables|Default|GetSphere) false true))))

(event EventBeginPlay)

(event Collision|EventActorBeginOverlap
  (params (OtherActor :type Actor%20Object%20Reference)))

(event EventTick
  (params (DeltaSeconds :type Float%20%28single-precision%29))
  (bind _initlocation (Variables|Default|GetInitLocation))
  (bind (_x _y _z) (Math|Vector|BreakVector _initlocation))
  (Variables|Default|SetSeconds (+ DeltaSeconds (Variables|Default|GetSeconds)))
  (Utilities|FlowControl|Sequence
    (:then_0
      (if (Variables|Default|GetHovering)
        (Transformation|SetActorLocation (Math|Vector|MakeVector _x _y (+ _z (* (+ (Math|Trig|Sin(Radians) (/ (Variables|Default|GetSeconds) (Variables|Default|GetPeriod))) 1.0) (Variables|Default|GetAmplitude)))) false false)))
    (:then_1
      (if (Variables|Default|GetRotating)
        (Transformation|SetActorRotation (Math|Rotator|MakeRotator 0.0 0.0 (* (Variables|Default|GetSeconds) (Variables|Default|GetRotationSpeed))))))))

(fn ConstructionScript
  (Variables|Default|SetInitLocation (Transformation|GetActorLocation)))