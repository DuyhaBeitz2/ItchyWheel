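; BP_LineGen is an environment Blueprint that builds a straight row of static meshes along its local X axis.
; The construction script places FirstMesh at the origin, then adds copies of Mesh for indices 1 through Size - 1.
; Each copy's offset is its index times the sum of Mesh's local X bounds and the Distance gap, ignoring FirstMesh's width.
; The event graph has no active logic.
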(event EventBeginPlay)

(event Collision|EventActorBeginOverlap
  (params (OtherActor :type Actor%20Object%20Reference)))

(event EventTick
  (params (DeltaSeconds :type Float%20%28single-precision%29)))

(fn ConstructionScript
  (bind _returnvalue (AddComponent|AddStaticMeshComponent false))
  (Components|StaticMesh|SetStaticMesh _returnvalue (Variables|Default|GetFirstMesh))
  (for _index (range 1 (- (Variables|Default|GetSize) 1))
    (bind _returnvalue_2 (AddComponent|AddStaticMeshComponent false))
    (Components|StaticMesh|SetStaticMesh _returnvalue_2 (Variables|Default|GetMesh))
    (Transformation|SetRelativeLocation _returnvalue_2 (Math|Vector|MakeVector (+ (.x (* (- (.Max (Components|StaticMesh|GetLocalBounds _returnvalue_2)) (.Min (Components|StaticMesh|GetLocalBounds _returnvalue_2))) _index)) (* _index (Variables|Default|GetDistance))) 0.0 0.0) false false)))