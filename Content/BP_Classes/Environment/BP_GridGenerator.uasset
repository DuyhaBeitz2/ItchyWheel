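; Grid generator actor that builds a rectangular tile layout from static meshes in its Construction Script.
; Nested loops over X/Y scale add a mesh component per tile, spaced by tile size, optionally leaving the interior empty.
; OnTheOutside flags border tiles using configurable widths, and OnTheAngle identifies four corner positions.
; These results select inner, edge or corner mesh and its rotation, with a separate rotation per corner.
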(event EventBeginPlay)

(event Collision|EventActorBeginOverlap
  (params (OtherActor :type Actor%20Object%20Reference)))

(event EventTick
  (params (DeltaSeconds :type Float%20%28single-precision%29)))

(fn ConstructionScript
  (bind _tilescale (Variables|Default|GetTileScale))
  (bind (_x _y) (Math|Vector|BreakVector _tilescale))
  ;[1 1 1] Loop
  (for _index (range 0 (- (Variables|Default|GetY_Scale) 1))
    (Variables|Default|Setindex_y _index)
    (for _index_2 (range 0 (- (Variables|Default|GetX_Scale) 1))
      (Variables|Default|Setindex_x _index_2)
      ;[1 1 1] Is on the outside
      (bind _ontheoutside (CallFunction|OntheOutside (Variables|Default|Getindex_x) (Variables|Default|Getindex_y)))
      (Variables|Default|SetOnOutside _ontheoutside)
      ;[1 1 1] On the angle
      (bind (_ontheangle _angleindex) (CallFunction|OntheAngle (Variables|Default|Getindex_x) (Variables|Default|Getindex_y)))
      (Variables|Default|SetOn%20the%20Angle _ontheangle)
      (Variables|Default|SetAngle%20Index _angleindex)
      ;[1 1 1] Is empty inside
      (if (or (Variables|Default|GetOnOutside) (not (Variables|Default|GetIsEmptyInside)))
        ;[1 1 1] Add new mesh component
        (bind _returnvalue (AddComponent|AddStaticMeshComponent false))
        (Variables|Default|SetNewMesh _returnvalue)
        ;[1 1 1] Location
        (Transformation|SetRelativeLocation (Variables|Default|GetNewMesh) (Math|Vector|MakeVector (* (Variables|Default|Getindex_x) _x) (* (Variables|Default|Getindex_y) _y) 0.0) false false)
        (Components|StaticMesh|SetStaticMesh (Variables|Default|GetNewMesh) (select (Variables|Default|GetOnOutside) (select (Variables|Default|GetOn%20the%20Angle) (Variables|Default|GetAngleMesh) (Variables|Default|GetOutSideMesh)) (Variables|Default|GetInnerMesh)))
        ;[1 1 1] Rotation
        (if (and (Variables|Default|GetOnOutside) (not (Variables|Default|GetOn%20the%20Angle)))
          ;;[1 1 1] Outside rotation
          (Transformation|AddRelativeRotation (Variables|Default|GetNewMesh) (Variables|Rotation|GetOutsideRotation) false false)
          (elif (Variables|Default|GetOn%20the%20Angle)
            ;;[1 1 1] Angle rotation
            (Transformation|AddRelativeRotation (Variables|Default|GetNewMesh) (Utilities|Select :Index (Variables|Default|GetAngle%20Index) :Option%200 "0, 0, 0" :Option%201 (Variables|Rotation|GetFirstAngleRotation) :Option%202 (Variables|Rotation|GetSecondAngleRotation) :Option%203 (Variables|Rotation|GetThirdAngleRotation) :Option%204 (Variables|Rotation|GetFourthAngleRotation)) false false)
            (else
              ;;[1 1 1] Inner rotation
              (Transformation|AddRelativeRotation (Variables|Default|GetNewMesh) (Variables|Rotation|GetInnerRotation) false false))))))))

(fn OntheOutside
  (params (X_Index :type Integer) (Y_Index :type Integer))
  (return (or (or (<= X_Index (Variables|Default|GetX_Width)) (<= Y_Index (Variables|Default|GetY_Width))) (or (>= X_Index (Utilities|Operators|Subtract (Variables|Default|GetX_Scale) (Variables|Default|GetX_Width) 1)) (>= Y_Index (Utilities|Operators|Subtract (Variables|Default|GetY_Scale) (Variables|Default|GetY_Width) 1))))))

(fn OntheAngle
  (params (X_Index :type Integer) (Y_Index :type Integer))
  ;[1 1 1] First angle
  (if (and (== X_Index 0) (== Y_Index 0))
    (return true 1)
    (else
      ;[1 1 1] Second angle
      (if (and (== X_Index 0) (== Y_Index (Utilities|Operators|Subtract (Variables|Default|GetY_Scale) (Variables|Default|GetY_Width) 1)))
        (return true 2)
        (else
          ;[1 1 1] Third angle
          (if (and (== X_Index (Utilities|Operators|Subtract (Variables|Default|GetX_Scale) (Variables|Default|GetX_Width) 1)) (== Y_Index 0))
            (return true 3)
            (else
              ;[1 1 1] Fourth angle
              (if (and (== X_Index (Utilities|Operators|Subtract (Variables|Default|GetX_Scale) (Variables|Default|GetX_Width) 1)) (== Y_Index (Utilities|Operators|Subtract (Variables|Default|GetY_Scale) (Variables|Default|GetY_Width) 1)))
                (return true 4)
                (else
                  ;[1 1 1] Not on the angle
                  (return false 0))))))))))