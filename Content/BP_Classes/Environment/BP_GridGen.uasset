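; BP_GridGen is an environment actor that builds a rectangular grid of static mesh components in its construction script.
; It loops over SizeX by SizeY cells, optionally leaving the inside empty so only a border of configurable width remains.
; PlaceMesh picks a corner, outside or inner mesh from each cell's position, spacing it by that mesh's local bounds plus Distance.
; Cells within the mesh border width on the X edges are rotated 90 degrees.
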(event EventBeginPlay)

(event Collision|EventActorBeginOverlap
  (params (OtherActor :type Actor%20Object%20Reference)))

(event EventTick
  (params (DeltaSeconds :type Float%20%28single-precision%29)))

(fn ConstructionScript
  (for _index (range 0 (- (Variables|Default|GetSizeY) 1))
    (for _index_2 (range 0 (- (Variables|Default|GetSizeX) 1))
      (|PlaceMesh _index_2 _index (Variables|Default|GetDistance)))))

(fn IsontheOutside
  (params (IndexX :type Integer) (IndexY :type Integer) (WidthX :type Integer) (WidthY :type Integer))
  (return (Math|Boolean|ORBoolean (>= IndexX (- (Variables|Default|GetSizeX) WidthX)) (<= IndexX (- WidthX 1)) (>= IndexY (- (Variables|Default|GetSizeY) WidthY)) (<= IndexY (- WidthY 1)))))

(fn IsontheAngle
  (params (IndexX :type Integer) (IndexY :type Integer))
  (return (and (or (== IndexX 0) (== IndexX (- (Variables|Default|GetSizeX) 1))) (or (== IndexY 0) (== IndexY (- (Variables|Default|GetSizeY) 1))))))