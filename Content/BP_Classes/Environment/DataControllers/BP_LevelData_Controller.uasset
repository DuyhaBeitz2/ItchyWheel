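; Level data controller that handles level completion, best times and star ratings for the level at LevelIndex.
; On completion it sends the next level index to the GameInstance, then shows the cached completion menu with UI-only input, or only creates it if missing.
; EvaluateLevelData merges results with saved data, with Stopwatch favoring longer times.
; GetStars checks Timings, sorted at construction, but its Stopwatch branch ignores Time.
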(event EventBeginPlay)

(event Collision|EventActorBeginOverlap
  (params (OtherActor :type Actor%20Object%20Reference)))

(event EventTick
  (params (DeltaSeconds :type Float%20%28single-precision%29)))

(event EventOnLevelComplete
  (Class|BPISaveGame|AddLevel(Message) (Game|GetGameInstance) false (+ (Variables|Default|GetLevelIndex) 1))
  ;[1 1 1] Add level complete widget
  (Utilities|IsValid (Variables|Default|GetCompleteLevelMenu)
    (:Is%20Valid
      (UserInterface|Viewport|AddtoViewport (stale _output_get) 0)
      (Input|SetInputModeUIOnly (Game|GetPlayerController 0) (Variables|Default|GetCompleteLevelMenu) "DoNotLock" false)
      (Variables|/Script/Engine.PlayerController|SetbShowMouseCursor (Game|GetPlayerController 0) true))
    (:Is%20Not%20Valid
      (bind _returnvalue (UserInterface|CreateWidget "/Game/UI/Menus/LevelComplete/WB_LevelCompleteMenu.WB_LevelCompleteMenu_C" (Game|GetPlayerController 0)))
      (bind _output_get (Variables|Default|SetCompleteLevelMenu _returnvalue)))))

(fn ConstructionScript
  (Class|KismetArrayLibrary|SortFloatArray (Variables|Default|GetTimings)))

(fn EvaluateLevelData
  (params (Time :type Float%20%28double-precision%29) (Stopwatch :type Boolean))
  (bind _savegamedata (Class|BPISaveGame|GetGameData(Message) (Game|GetGameInstance)))
  (if (== (.BestTime (Utilities|Struct|BreakS_LevelData (Utilities|Array|Get(acopy) (Variables|/Game/Saves/BP_SaveGame.BP_SaveGame_C|GetLevelData _savegamedata) (Variables|Default|GetLevelIndex)))) 0.0)
    (bind _stars (CallFunction|GetStars Time Stopwatch))
    (return (Utilities|Struct|MakeS_LevelData Time (Math|Integer|Max(Integer) _stars (.Stars (Utilities|Struct|BreakS_LevelData (Utilities|Array|Get(acopy) (Variables|/Game/Saves/BP_SaveGame.BP_SaveGame_C|GetLevelData _savegamedata) (Variables|Default|GetLevelIndex)))))))
    (else
      (bind _stars_2 (CallFunction|GetStars Time Stopwatch))
      (return (Utilities|Struct|MakeS_LevelData (Math|Float|SelectFloat (Math|Float|Max(Float) (.BestTime (Utilities|Struct|BreakS_LevelData (Utilities|Array|Get(acopy) (Variables|/Game/Saves/BP_SaveGame.BP_SaveGame_C|GetLevelData _savegamedata) (Variables|Default|GetLevelIndex)))) Time) (Math|Float|Min(Float) (.BestTime (Utilities|Struct|BreakS_LevelData (Utilities|Array|Get(acopy) (Variables|/Game/Saves/BP_SaveGame.BP_SaveGame_C|GetLevelData _savegamedata) (Variables|Default|GetLevelIndex)))) Time) Stopwatch) (Math|Integer|Max(Integer) _stars_2 (.Stars (Utilities|Struct|BreakS_LevelData (Utilities|Array|Get(acopy) (Variables|/Game/Saves/BP_SaveGame.BP_SaveGame_C|GetLevelData _savegamedata) (Variables|Default|GetLevelIndex))))))))))

(fn GetStars
  (params (Time :type Float%20%28double-precision%29) (Stopwatch :type Boolean))
  (if Stopwatch
    (bind (_arrayindex _arrayelement) (Utilities|Array|ReverseforEachLoop (Variables|Default|GetTimings))
      (:LoopBody
        (if true
          (return (- 3 _arrayindex))))
      (:Completed
        (return 0)))
    (else
      (for (_array_element _array_index) (Variables|Default|GetTimings)
        (if (<= Time _array_element)
          (return (- 3 _array_index))))
      (return 0))))