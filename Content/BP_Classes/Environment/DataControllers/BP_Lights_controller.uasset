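; BP_Lights_controller is an environment data controller that sets the light state of vehicles, lamps and buildings across the level from a single LightsOn value.
; When UpdateObjects is true, its Construction Script finds every BP_VehicleAI, BP_Lamp_01 and BP_BuildingGen actor and copies LightsOn onto each.
; The Event Graph holds only disabled placeholder events, so the propagation runs only on construction, not during BeginPlay or Tick.
; It only writes the variable and calls no refresh on those actors.
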(event EventBeginPlay)

(event Collision|EventActorBeginOverlap
  (params (OtherActor :type Actor%20Object%20Reference)))

(event EventTick
  (params (DeltaSeconds :type Float%20%28single-precision%29)))

(fn ConstructionScript
  (if (Variables|Default|GetUpdateObjects)
    (Utilities|FlowControl|Sequence
      (:then_0
        ;[1 1 1] Vehicles
        (bind _outactors (Actor|GetAllActorsOfClass "/Game/BP_Classes/Cars/BP_VehicleAI.BP_VehicleAI_C"))
        (for _array_element _outactors
          (Variables|/Game/BP_Classes/Cars/BP_VehicleAI.BP_VehicleAI_C|SetLightsOn _array_element (Variables|Default|GetLightsOn))))
      (:then_1
        ;[1 1 1] Lamps
        (bind _outactors_2 (Actor|GetAllActorsOfClass "/Game/Environment/Props/Lamp_01/BP_Lamp_01.BP_Lamp_01_C"))
        (for _array_element_2 _outactors_2
          (Variables|/Game/Environment/Props/Lamp_01/BP_Lamp_01.BP_Lamp_01_C|SetLightsOn _array_element_2 (Variables|Default|GetLightsOn))))
      (:then_2
        ;[1 1 1] Lamps
        (bind _outactors_3 (Actor|GetAllActorsOfClass "/Game/Environment/Buildings/BP_BuildingGen.BP_BuildingGen_C"))
        (for _array_element_3 _outactors_3
          (Variables|/Game/Environment/Buildings/BP_BuildingGen.BP_BuildingGen_C|SetLightsOn _array_element_3 (Variables|Default|GetLightsOn)))))))