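; BP_Timer is the level timer, counting Seconds on Tick while Going: down if StopWatch is true, up otherwise.
; TimePunishment and TimeReward adjust the running time according to that direction and display the signed change in reused widgets.
; Start and Stop only set Going, while ToggleGoing, when halting a running timer, also saves level data evaluated through BP_LevelData_Controller and notifies it and the player's BP_VehicleAI of level completion.
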(event EventBeginPlay)

(event EventTick
  (params (DeltaSeconds :type Float%20%28single-precision%29))
  (if (Variables|Default|GetGoing)
    (if (Variables|Default|GetStopWatch)
      (Variables|Default|SetSeconds (- (Variables|Default|GetSeconds) DeltaSeconds))
      (else
        (Variables|Default|SetSeconds (+ (Variables|Default|GetSeconds) DeltaSeconds))))))

(fn ConstructionScript)

(fn TimePunishment
  (params (AbsAmount :type Float%20%28double-precision%29))
  (bind _returnvalue (* AbsAmount -1.0))
  (if (Variables|Default|GetGoing)
    (if (Variables|Default|GetStopWatch)
      (Variables|Default|SetSeconds (+ (Variables|Default|GetSeconds) _returnvalue))
      (Utilities|IsValid (Variables|Default|GetPunishWidget)
        (:Is%20Valid
          _)
        (:Is%20Not%20Valid
          (bind _returnvalue_2 (UserInterface|CreateWidget "/Game/UI/HUD/TimePunshmentWidget/WB_TimePunishment.WB_TimePunishment_C" (Game|GetPlayerController 0)))
          (Variables|Default|SetPunishWidget _returnvalue_2)))
      (Default|SetTimeAmount (Variables|Default|GetPunishWidget) _returnvalue)
      (UserInterface|Viewport|AddtoViewport (Variables|Default|GetPunishWidget) 0)
      (else
        (Variables|Default|SetSeconds (+ (Variables|Default|GetSeconds) AbsAmount))
        (Utilities|IsValid (Variables|Default|GetPunishWidget)
          (:Is%20Valid
            _)
          (:Is%20Not%20Valid
            (bind _returnvalue_3 (UserInterface|CreateWidget "/Game/UI/HUD/TimePunshmentWidget/WB_TimePunishment.WB_TimePunishment_C" (Game|GetPlayerController 0)))
            (Variables|Default|SetPunishWidget _returnvalue_3)))
        (Default|SetTimeAmount (Variables|Default|GetPunishWidget) AbsAmount)
        (UserInterface|Viewport|AddtoViewport (Variables|Default|GetPunishWidget) 0)))))

(fn Stop
  (Variables|Default|SetGoing false))

(fn Start
  (Variables|Default|SetGoing true))

(fn ToggleGoing
  (Utilities|FlowControl|Sequence
    (:then_0
      ;[1 1 1] Save if was going
      (if (Variables|Default|GetGoing)
        (bind _returnvalue (Actor|GetActorOfClass "/Game/BP_Classes/Environment/DataControllers/BP_LevelData_Controller.BP_LevelData_Controller_C"))
        (bind _leveldata (Default|EvaluateLevelData _returnvalue (Variables|Default|GetSeconds) (not (Variables|Default|GetStopWatch))))
        (Class|BPISaveGame|SaveLevelData(Message) (Game|GetGameInstance) false _leveldata (Variables|/Game/BP_Classes/Environment/DataControllers/BP_LevelData_Controller.BP_LevelData_Controller_C|GetLevelIndex _returnvalue))
        (Default|OnLevelComplete _returnvalue)
        (bind _asbp_vehicle_ai (Utilities|Casting|CastToBP_VehicleAI (Game|Player|GetPlayerPawn 0)))
        (Default|OnLevelComplete _asbp_vehicle_ai)))
    (:then_1
      (Variables|Default|SetGoing (not (Variables|Default|GetGoing))))))

(fn TimeReward
  (params (AbsAmount :type Float%20%28double-precision%29))
  (bind _returnvalue (* AbsAmount -1.0))
  (if (Variables|Default|GetGoing)
    (if (Variables|Default|GetStopWatch)
      (Variables|Default|SetSeconds (+ (Variables|Default|GetSeconds) AbsAmount))
      (Utilities|IsValid (Variables|Default|GetRewardWidget)
        (:Is%20Valid
          _)
        (:Is%20Not%20Valid
          (bind _returnvalue_2 (UserInterface|CreateWidget "/Game/UI/HUD/TimeRewardWidget/WB_TimeReward.WB_TimeReward_C" (Game|GetPlayerController 0)))
          (Variables|Default|SetRewardWidget _returnvalue_2)))
      (UserInterface|Viewport|AddtoViewport (Variables|Default|GetRewardWidget) 0)
      (Default|SetTimeAmount (Variables|Default|GetRewardWidget) AbsAmount)
      (else
        (Variables|Default|SetSeconds (+ (Variables|Default|GetSeconds) _returnvalue))
        (Utilities|IsValid (Variables|Default|GetRewardWidget)
          (:Is%20Valid
            _)
          (:Is%20Not%20Valid
            (bind _returnvalue_3 (UserInterface|CreateWidget "/Game/UI/HUD/TimeRewardWidget/WB_TimeReward.WB_TimeReward_C" (Game|GetPlayerController 0)))
            (Variables|Default|SetRewardWidget _returnvalue_3)))
        (UserInterface|Viewport|AddtoViewport (Variables|Default|GetRewardWidget) 0)
        (Default|SetTimeAmount (Variables|Default|GetRewardWidget) _returnvalue)))))