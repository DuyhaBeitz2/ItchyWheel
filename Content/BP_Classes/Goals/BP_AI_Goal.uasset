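; BP_AI_Goal is a waypoint actor that guides BP_AI_Car vehicles along a chain of goals.
; When a car targeting this goal overlaps the Sphere, it receives GoalReached with the next goal and a final-goal flag.
; If ForceSlowDown is enabled, overlapping SlowDownSphere makes that car slow down.
; The construction script rotates an Arrow toward NextGoal to show the route direction.
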(event OnComponentBeginOverlap(Sphere)
  (params (OverlappedComponent :type Primitive%20Component%20Object%20Reference) (OtherActor :type Actor%20Object%20Reference) (OtherComp :type Primitive%20Component%20Object%20Reference) (OtherBodyIndex :type Integer) (bFromSweep :type Boolean) (SweepResult :type Hit%20Result%20Structure%20%28by%20ref%29))
  (bind _asbp_ai_car (Utilities|Casting|CastToBP_AI_Car OtherActor))
  (if (== (Variables|/Game/BP_Classes/Cars/BP_AI_Car.BP_AI_Car_C|GetGoal _asbp_ai_car) self)
    (Default|GoalReached _asbp_ai_car (Variables|Goal|GetNextGoal) (Variables|Goal|GetFinalGoal))))

(event OnComponentBeginOverlap(SlowDownSphere)
  (params (OverlappedComponent :type Primitive%20Component%20Object%20Reference) (OtherActor :type Actor%20Object%20Reference) (OtherComp :type Primitive%20Component%20Object%20Reference) (OtherBodyIndex :type Integer) (bFromSweep :type Boolean) (SweepResult :type Hit%20Result%20Structure%20%28by%20ref%29))
  (if (Variables|Goal|GetForceSlowDown)
    (bind _asbp_ai_car (Utilities|Casting|CastToBP_AI_Car OtherActor))
    (if (== (Variables|/Game/BP_Classes/Cars/BP_AI_Car.BP_AI_Car_C|GetGoal _asbp_ai_car) self)
      (Default|ForceSlowDown _asbp_ai_car))))

(event EventBeginPlay)

(event Collision|EventActorBeginOverlap
  (params (OtherActor :type Actor%20Object%20Reference)))

(event EventTick
  (params (DeltaSeconds :type Float%20%28single-precision%29)))

(fn ConstructionScript
  (Transformation|SetWorldRotation (Variables|Default|GetArrow) (Math|Rotator|FindLookatRotation (Transformation|GetActorLocation) (Transformation|GetActorLocation (Variables|Goal|GetNextGoal))) false false))